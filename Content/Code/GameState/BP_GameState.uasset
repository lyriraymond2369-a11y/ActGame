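; Game state that runs a token pool limiting how many actors, likely enemies, can hold a token at once.
; AddToken grants timestamped tokens subject to the current cap and a cooldown since the last release, while HasToken and RemoveToken query and free them.
; A throttled Tick purges invalid, dead or timed-out holders, then sets the cap to one below the living enemy count, clamped to a small range.
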(event Custom|UpdateTokens
  ;[0.15 0.15 0.15 0.5 36] 更新
  (Utilities|Array|Clear (Variables|Default|GetBadTokens))
  (Utilities|FlowControl|Sequence
    (:then_0
      (bind (_keypin _valuepin) (Utilities|Map|ForEachLoop(Map) (Variables|Default|GetTokens))
        (:then
          (Variables|中间变量|SetMiddleActor _keypin)
          (Variables|中间变量|SetMiddleFloat _valuepin)
          (Utilities|FlowControl|Sequence
            (:then_0
              (Utilities|IsValid (Variables|中间变量|GetMiddleActor)
                (:Is%20Not%20Valid
                  (Utilities|Array|AddUnique (Variables|Default|GetBadTokens) (Variables|中间变量|GetMiddleActor)))))
            (:then_1
              (bind _rezult (Class|BPICharacterBase|IsCharacterDead(Message) (Variables|中间变量|GetMiddleActor)))
              (if _rezult
                (Utilities|Array|AddUnique (Variables|Default|GetBadTokens) (Variables|中间变量|GetMiddleActor))))
            (:then_2
              (if (>= (- (Utilities|Time|GetGameTimeinSeconds) (Variables|中间变量|GetMiddleFloat)) (Variables|Default|GetTokenTimeout))
                (Utilities|Array|AddUnique (Variables|Default|GetBadTokens) (Variables|中间变量|GetMiddleActor))))))))
    (:then_1
      (for _array_element (Variables|Default|GetBadTokens)
        (CallFunction|RemoveToken _array_element)))))

(event Custom|UpdateMaxToken
  ;[0.15 0.15 0.15 0.5 36] 更新
  (Variables|Default|SetAliveCount 0)
  (bind _outactors (Actor|GetAllActorsOfClass "/Game/Enemy/BP_EnemyBase.BP_EnemyBase_C"))
  (for _array_element _outactors
    (Utilities|IsValid _array_element
      (:Is%20Valid
        (bind _rezult (Class|BPICharacterBase|IsCharacterDead(Message) _array_element))
        (if (not _rezult)
          (Math|Integer|IncrementInt (Variables|Default|GetAliveCount))))))
  (Variables|Default|SetMaxToken (Math|Integer|Clamp(Integer) (- (Variables|Default|GetAliveCount) 1) 1 2)))

(event EventBeginPlay
  (Actor|Tick|SetActorTickInterval (Variables|Default|GetCleanupInterval)))

(event EventTick
  (params (DeltaSeconds :type Float%20%28single-precision%29))
  (CallFunction|UpdateTokens)
  (CallFunction|UpdateMaxToken))

(event EventRemoveToken
  (params (Holder :type Actor%20Object%20Reference))
  ;[0.15 0.15 0.15 0.5 36] 接口事件
  (Variables|中间变量|SetMiddleActor Holder)
  (if (Utilities|Map|Contains (Variables|Default|GetTokens) (Variables|中间变量|GetMiddleActor))
    (Utilities|Map|Remove (Variables|Default|GetTokens) (Variables|中间变量|GetMiddleActor))
    (Variables|Default|SetLastReleaseTime (Utilities|Time|GetGameTimeinSeconds))))

(fn ConstructionScript)

(fn AddToken
  (params (Actor :type Actor%20Object%20Reference))
  (LocalVariables|SetHolder Actor)
  (Utilities|FlowControl|Sequence
    (:then_0
      (Utilities|IsValid (LocalVariables|GetHolder)
        (:Is%20Not%20Valid
          (return false))))
    (:then_1
      (if (Utilities|Map|Contains (Variables|Default|GetTokens) (LocalVariables|GetHolder))
        (return true)))
    (:then_2
      (if (>= (Utilities|Map|Length (Variables|Default|GetTokens)) (Variables|Default|GetMaxToken))
        (return false)))
    (:then_3
      (if (< (- (Utilities|Time|GetGameTimeinSeconds) (Variables|Default|GetLastReleaseTime)) (Variables|Default|GetTokenCooldown))
        (return false)))
    (:then_4
      (Utilities|Map|Add (Variables|Default|GetTokens) (LocalVariables|GetHolder) (Utilities|Time|GetGameTimeinSeconds))
      (return true))))

(fn HasToken
  (params (actor :type Actor%20Object%20Reference))
  (return (Utilities|Map|Contains (Variables|Default|GetTokens) actor)))