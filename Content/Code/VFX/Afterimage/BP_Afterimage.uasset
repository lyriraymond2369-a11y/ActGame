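; BP_Afterimage is a ghost afterimage actor that shows a frozen pose of a skeletal mesh and fades out.
; An interface event, CopyPosefrom, copies the target mesh's pose onto its PoseableMesh.
; On BeginPlay it applies one dynamic instance of GhostMaterial to every material slot, while a timeline lowers Opacity.
; The actor destroys itself when the fade finishes.
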(event EventBeginPlay
  (bind _returnvalue (Rendering|Material|CreateDynamicMaterialInstance (Variables|Default|GetGhostMaterial) "None" "Transient" :!class /Script/Engine.KismetMaterialLibrary))
  (Variables|Default|SetMID _returnvalue)
  (Utilities|FlowControl|Sequence
    (:then_0
      (for _index (range 0 (- (Rendering|Material|GetNumMaterials (Variables|Default|GetPoseableMesh)) 1))
        (Rendering|Material|SetMaterial (Variables|Default|GetPoseableMesh) _index (Variables|Default|GetMID))))
    (:then_1
      (bind _alpha (Timeline|TL_Fade PlayFromStart)
        (:Update
          (Rendering|Material|SetScalarParameterValue (Variables|Default|GetMID) "Opacity" (- 1.0 _alpha) :!class /Script/Engine.MaterialInstanceDynamic))
        (:Finished
          (Actor|DestroyActor))))))

(event EventCopyPosefrom
  (params (TargetMesh :type Skeletal%20Mesh%20Component%20Object%20Reference))
  ;[0.15 0.15 0.15 0.5 36] 接口事件
  (Class|PoseableMeshComponent|CopyPosefromSkeletalComponent (Variables|Default|GetPoseableMesh) TargetMesh))

(event EventTick
  (params (DeltaSeconds :type Float%20%28single-precision%29)))

(fn ConstructionScript)