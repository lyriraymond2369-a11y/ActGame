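; BP_Slash is a self-destroying slash VFX actor built on a static mesh with a dynamic material.
; BeginPlay creates the material instance, applies color and start scale, then plays the T_Opacity timeline.
; Each update fades opacity by inverse alpha, multiplies current scale by a start-to-end lerp and adds alpha-weighted sweep to current yaw, so both compound per frame.
; The actor destroys itself when the timeline finishes.
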(event EventBeginPlay
  (bind _returnvalue (Transformation|GetActorRotation))
  (bind _returnvalue_2 (Rendering|Material|CreateDynamicMaterialInstance (Variables|Default|GetSlashMaterial) "None" "None" :!class /Script/Engine.KismetMaterialLibrary))
  (bind _output_get (Variables|Default|SetMID _returnvalue_2))
  (Rendering|Material|SetMaterial (Variables|Default|GetStaticMesh) 0 _output_get)
  (Utilities|FlowControl|Sequence
    (:then_0
      (Rendering|Material|SetVectorParameterValue (Variables|Default|GetMID) "Color" (Variables|Default|GetColor) :!class /Script/Engine.MaterialInstanceDynamic)
      (Rendering|Material|SetScalarParameterValue (Variables|Default|GetMID) (Variables|Default|GetOpacityName) (Variables|Default|GetStartScale) :!class /Script/Engine.MaterialInstanceDynamic))
    (:then_1
      (Transformation|SetActorScale3D (* (Transformation|GetActorScale3D) (Variables|Default|GetStartScale)))
      (bind _alpha (Timeline|T_Opacity PlayFromStart)
        (:Update
          (Variables|Default|SetAlpha _alpha)
          (Transformation|SetActorScale3D (* (Transformation|GetActorScale3D) (Math|Float|Lerp (Variables|Default|GetStartScale) (Variables|Default|GetEndScale) (Variables|Default|GetAlpha))))
          (Rendering|Material|SetScalarParameterValue (Variables|Default|GetMID) (Variables|Default|GetOpacityName) (- 1.0 (Variables|Default|GetAlpha)) :!class /Script/Engine.MaterialInstanceDynamic)
          (Transformation|SetActorRotation (Math|Rotator|MakeRotator (.roll _returnvalue) (.pitch _returnvalue) (+ (.yaw _returnvalue) (* (Variables|Default|GetAlpha) (Variables|Default|GetSweepAngle))))))
        (:Finished
          (Actor|DestroyActor))))))

(fn ConstructionScript)