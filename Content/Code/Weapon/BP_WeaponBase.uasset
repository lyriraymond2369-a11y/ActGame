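; Base weapon Blueprint that supplies a hit box, a bonus value and a toggleable Niagara trail effect.
; SetTrailActive compares the requested state with TrailActive and activates or deactivates the Niagara component only when the state changes.
; GetWeaponBonus and GetWeaponHitBox expose the bonus and Box component to other code, and the Blueprint itself contains no hit or damage logic.
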(event EventBeginPlay)

(event Collision|EventActorBeginOverlap
  (params (OtherActor :type Actor%20Object%20Reference)))

(event EventTick
  (params (DeltaSeconds :type Float%20%28single-precision%29)))

(event EventSetTrailActive
  (params (Val :type Boolean))
  (bind _output_get (Variables|中间变量|SetMiddleBool Val))
  (if (Class|KismetMathLibrary|XORBoolean _output_get (Variables|Default|GetbTrailActive))
    (bind _output_get_2 (Variables|Default|SetbTrailActive (Variables|中间变量|GetMiddleBool)))
    (if _output_get_2
      (Components|Activation|Activate (Variables|Default|GetNiagara) false)
      (else
        (Components|Activation|Deactivate (Variables|Default|GetNiagara))))))

(fn ConstructionScript)

(fn GetWeaponBonus
  (return (Variables|默认|GetWeaponBonus)))

(fn GetWeaponHitBox
  (return (Variables|Default|GetBox)))