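; Actor component that plays combat feedback for hit, block, guard break and posture break outcomes while its owner is alive.
; Each outcome combines sound, a timed hit stop freezing both actors via CustomTimeDilation, and CameraDirector shakes or cinematic effects.
; Posture breaks queue local slow motion, which Tick starts on the owner once hit stop ends.
; It also provides timed slow motion for all enemies and perfect block, dodge and grab sounds.
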(event Custom|PlayPerfectDodgeEndSound
  ;[0.15 0.15 0.15 0.5 36] 中间事件
  (Audio|PlaySound2D (Variables|音效|GetPerfectDodgeEndSound) 1.0 1.0 0.0 0 0))

(event Custom|RestoreSlowMo
  ;[0.15 0.15 0.15 0.5 36] 中间事件
  (for _array_element (Variables|放缓|GetSlowMoActors)
    (Utilities|IsValid _array_element
      (:Is%20Valid
        (Variables|/Script/Engine.Actor|SetCustomTimeDilation _array_element 1.0))))
  (Utilities|Array|Clear (Variables|放缓|GetSlowMoActors))
  (Utilities|Time|SetGlobalTimeDilation 1.0))

(event Custom|UpdateSlowMo
  ;[0.15 0.15 0.15 0.5 36] 更新
  (if (Math|Boolean|ANDBoolean (> (Variables|时间膨胀|GetPendingSlowMoDuration) 0.0) (not (Variables|顿帧|GetbInHitStop)) (== (Variables|/Script/Engine.Actor|GetCustomTimeDilation (Variables|Default|GetOwner)) (Variables|时间膨胀|GetLocalSlowMoOriginalDilation)))
    (CallFunction|StartLocalSlowMo)))

(event Custom|HandleGuardHitFeedback
  (params (ImpactLocation :type Vector) (BaseHitStop :type Float%20%28double-precision%29) (OtherActor :type Actor%20Object%20Reference) (Perfect :type Boolean))
  ;[0.15 0.15 0.15 0.5 36] 中间事件
  (Variables|中间变量|SetMiddleVector3 ImpactLocation)
  (Variables|中间变量|SetMiddleFloat BaseHitStop)
  (Variables|中间变量|SetMiddleActor OtherActor)
  (Variables|中间变量|SetMiddleBool Perfect)
  (Audio|PlaySoundatLocation (Variables|音效|GetS_Block) (Variables|中间变量|GetMiddleVector3) "0, 0, 0" 1.0 1.0 0.0 0 0 0 0)
  (Utilities|FlowControl|Sequence
    (:then_0
      (if (Variables|中间变量|GetMiddleBool)
        (CallFunction|PlayHitStop (Variables|中间变量|GetMiddleActor) (* (Variables|中间变量|GetMiddleFloat) 2.0))
        (else
          (CallFunction|PlayHitStop (Variables|中间变量|GetMiddleActor) (Variables|中间变量|GetMiddleFloat)))))
    (:then_1
      (Class|BPICameraDirector|Shake(Message) (Variables|Default|GetCamera%20Director) (select (Variables|中间变量|GetMiddleBool) "NewEnumerator2" "NewEnumerator1") (Variables|中间变量|GetMiddleVector3) (select (Variables|中间变量|GetMiddleBool) 1.5 1.0)))
    (:then_2
      (if (and (Utilities|Enum|Equal(Enum) (Variables|中间变量|GetMiddleEnum) "NewEnumerator2") (Variables|中间变量|GetMiddleBool))
        (Class|BPICameraDirector|PlayPerfectBlockCloseUp(Message) (Variables|Default|GetCamera%20Director))))))

(event Custom|HandleGuardBreakFeedback
  (params (ImpactLocation :type Vector) (OtherActor :type Actor%20Object%20Reference))
  ;[0.15 0.15 0.15 0.5 36] 中间事件
  (Variables|中间变量|SetMiddleVector3 ImpactLocation)
  (Variables|中间变量|SetMiddleActor OtherActor)
  (Audio|PlaySoundatLocation (Variables|音效|GetS_PoiseBreak) (Variables|中间变量|GetMiddleVector3) "0, 0, 0" (Variables|Default|GetPoiseBreakVolume) 1.0 0.0 0 0 0 0)
  (CallFunction|PlayHitStop (Variables|中间变量|GetMiddleActor) 0.2)
  (Class|BPICameraDirector|Shake(Message) (Variables|Default|GetCamera%20Director) "NewEnumerator3" (Variables|中间变量|GetMiddleVector3) 1.0))

(event Custom|HandleNormalHitFeedback
  (params (ImpactLocation :type Vector) (BaseHitStop :type Float%20%28double-precision%29) (OtherActor :type Actor%20Object%20Reference))
  ;[0.15 0.15 0.15 0.5 36] 中间事件
  (Variables|中间变量|SetMiddleVector3 ImpactLocation)
  (Variables|中间变量|SetMiddleFloat BaseHitStop)
  (Variables|中间变量|SetMiddleActor OtherActor)
  (Audio|PlaySoundatLocation (Variables|音效|GetS_Hit) (Variables|中间变量|GetMiddleVector3) "0, 0, 0" 1.0 1.0 0.0 0 0 0 0)
  (CallFunction|PlayHitStop (Variables|中间变量|GetMiddleActor) (Variables|中间变量|GetMiddleFloat))
  (Class|BPICameraDirector|Shake(Message) (Variables|Default|GetCamera%20Director) "NewEnumerator0" (Variables|中间变量|GetMiddleVector3) 1.0))

(event Custom|HandleKnockdownFeedback
  (params (ImpactLocation :type Vector) (OtherActor :type Actor%20Object%20Reference) (BaseHitStop :type Float%20%28double-precision%29))
  ;[0.15 0.15 0.15 0.5 36] 中间事件
  (Variables|中间变量|SetMiddleVector3 ImpactLocation)
  (Variables|中间变量|SetMiddleActor OtherActor)
  (Variables|中间变量|SetMiddleFloat BaseHitStop)
  (CallFunction|PlayKnockdownSound)
  (Class|BPICameraDirector|Shake(Message) (Variables|Default|GetCamera%20Director) "NewEnumerator6" (Variables|中间变量|GetMiddleVector3) 2.0)
  (Class|BPICameraDirector|PlayKnockdownFOV(Message) (Variables|Default|GetCamera%20Director))
  (CallFunction|PlayHitStop (Variables|中间变量|GetMiddleActor) (Variables|中间变量|GetMiddleFloat))
  (CallFunction|PlayLocalSlowMo 0.25 0.5 (Variables|中间变量|GetMiddleActor)))

(event Custom|StartLocalSlowMo
  ;[0.15 0.15 0.15 0.5 36] 中间事件
  (Utilities|Time|ClearandInvalidateTimerbyHandle (Variables|时间膨胀|GetLocalSlowMoTimerHandle))
  (Variables|/Script/Engine.Actor|SetCustomTimeDilation (Variables|Default|GetOwner) (Variables|时间膨胀|GetPendingSlowMoScale))
  (bind _returnvalue (Utilities|Time|SetTimerbyEvent (delegate Custom|RestoreLocalSlowMo) (Variables|时间膨胀|GetPendingSlowMoDuration)))
  (Variables|时间膨胀|SetLocalSlowMoTimerHandle _returnvalue))

(event Custom|RestoreLocalSlowMo
  ;[0.15 0.15 0.15 0.5 36] 中间事件
  (Variables|/Script/Engine.Actor|SetCustomTimeDilation (Variables|Default|GetOwner) (Variables|时间膨胀|GetLocalSlowMoOriginalDilation))
  (Variables|/Script/Engine.Actor|SetCustomTimeDilation (Variables|时间膨胀|GetSlowOtherActor) (Variables|时间膨胀|GetLocalSlowMoOriginalDilation))
  (Utilities|Time|ClearandInvalidateTimerbyHandle (Variables|时间膨胀|GetLocalSlowMoTimerHandle))
  (Variables|时间膨胀|SetPendingSlowMoScale 0.0)
  (Variables|时间膨胀|SetPendingSlowMoDuration 0.0))

(event EventBeginPlay
  (bind _output_get (Variables|Default|SetOwner (Components|GetOwner)))
  (bind _attribute (Class|BPICharacterBase|GetAttributeComponent(Message) _output_get))
  (Variables|Default|SetAttribute _attribute)
  (bind _cameradirector (Class|BPIPlayer|GetCameraDirectorComponent(Message) (Game|Player|GetPlayerPawn 0)))
  (Variables|Default|SetCamera%20Director _cameradirector))

(event EventTick
  (params (DeltaSeconds :type Float%20%28single-precision%29))
  (CallFunction|UpdateSlowMo))

(event EventPlayLocalSlowMo
  (params (Scale :type Float%20%28double-precision%29) (Duration :type Float%20%28double-precision%29) (other :type Actor%20Object%20Reference))
  ;[0.15 0.15 0.15 0.5 36] 接口事件
  (Variables|时间膨胀|SetPendingSlowMoScale Scale)
  (Variables|时间膨胀|SetPendingSlowMoDuration Duration)
  (Variables|时间膨胀|SetSlowOtherActor other)
  (if (Math|Boolean|NORBoolean (>= (Variables|时间膨胀|GetPendingSlowMoScale) 1.0) (<= (Variables|时间膨胀|GetPendingSlowMoDuration) 0.0))
    (if (>= (Utilities|Time|GetGameTimeinSeconds) (Variables|顿帧|GetHitStopEndTime))
      (CallFunction|ApplyLocalSlowMo 0.25 0.5)
      (bind _feedback (Class|BPICharacterBase|GetCombatFeedbackComponent(Message) (Variables|时间膨胀|GetSlowOtherActor)))
      (Class|BPICombatFeedBack|ApplyLocalSlowMo(Message) _feedback 0.25 0.5))))

(event EventApplyLocalSlowMo
  (params (Scale :type Float%20%28double-precision%29) (Duration :type Float%20%28double-precision%29))
  ;[0.15 0.15 0.15 0.5 36] 接口事件
  (Variables|时间膨胀|SetPendingSlowMoScale Scale)
  (bind _output_get (Variables|时间膨胀|SetPendingSlowMoDuration Duration))
  (if (> _output_get 0.0)
    (if (not (Variables|顿帧|GetbInHitStop))
      (CallFunction|StartLocalSlowMo))))

(event EventPlayHitFeedback
  (params (Outcome :type E_HitOutCome%20Enum :default "NewEnumerator0") (ImpactLocation :type Vector :default "0, 0, 0") (bPerfect :type Boolean) (OtherActor :type Actor%20Object%20Reference) (BaseHitStop :type Float%20%28double-precision%29))
  ;[0.15 0.15 0.15 0.5 36] 接口事件
  (Variables|中间变量|SetMiddleEnum Outcome)
  (Variables|中间变量|SetMiddleVector3 ImpactLocation)
  (Variables|中间变量|SetMiddleBool bPerfect)
  (Variables|中间变量|SetMiddleActor OtherActor)
  (Variables|中间变量|SetMiddleFloat BaseHitStop)
  (bind _dead (Class|BPIAttribute|IsDead(Message) (Variables|Default|GetAttribute)))
  (if (not _dead)
    (Utilities|FlowControl|Sequence
      (:then_0
        (switch Utilities|FlowControl|Switch|SwitchonE_HitOutCome (Variables|中间变量|GetMiddleEnum)
          (:NewEnumerator1
            (CallFunction|HandleNormalHitFeedback (Variables|中间变量|GetMiddleVector3) (Variables|中间变量|GetMiddleFloat) (Variables|中间变量|GetMiddleActor)))
          (:NewEnumerator2
            (CallFunction|HandleGuardHitFeedback (Variables|中间变量|GetMiddleVector3) (Variables|中间变量|GetMiddleFloat) (Variables|中间变量|GetMiddleActor) (Variables|中间变量|GetMiddleBool)))
          (:NewEnumerator5
            (CallFunction|HandleGuardBreakFeedback (Variables|中间变量|GetMiddleVector3) (Variables|中间变量|GetMiddleActor)))
          (:NewEnumerator6
            (CallFunction|HandleKnockdownFeedback (Variables|中间变量|GetMiddleVector3) (Variables|中间变量|GetMiddleActor) 0.2)))))))

(event EventPlayHitStop
  (params (OtherActor :type Actor%20Object%20Reference) (Duration :type Float%20%28double-precision%29))
  ;[0.15 0.15 0.15 0.5 36] 接口事件
  (Variables|中间变量|SetMiddleActor OtherActor)
  (Variables|中间变量|SetMiddleFloat Duration)
  (if (and (Utilities|IsValid (Variables|中间变量|GetMiddleActor)) (> (Variables|中间变量|GetMiddleFloat) 0.0))
    (if (Variables|顿帧|GetbInHitStop)
      (Variables|顿帧|SetHitStopEndTime (Math|Float|Max(Float) (+ (Utilities|Time|GetGameTimeinSeconds) (Variables|中间变量|GetMiddleFloat)) (Variables|顿帧|GetHitStopEndTime)))
      (Utilities|Time|ClearandInvalidateTimerbyHandle (Variables|Default|GetTimerHandler))
      (bind _returnvalue (Utilities|Time|SetTimerbyEvent (EventDispatchers|CreateEvent :!event EndHitStop) (- (Variables|顿帧|GetHitStopEndTime) (Utilities|Time|GetGameTimeinSeconds))))
      (Variables|Default|SetTimerHandler _returnvalue)
      (else
        (Variables|顿帧|SetHitStopEndTime (+ (Utilities|Time|GetGameTimeinSeconds) (Variables|中间变量|GetMiddleFloat)))
        (Variables|顿帧|SetbInHitStop true)
        (Variables|顿帧|SetHitStopAttacker (Variables|Default|GetOwner))
        (Variables|顿帧|SetHitStopDefender (Variables|中间变量|GetMiddleActor))
        (Variables|/Script/Engine.Actor|SetCustomTimeDilation (Variables|Default|GetOwner) 0.0)
        (Variables|/Script/Engine.Actor|SetCustomTimeDilation (Variables|中间变量|GetMiddleActor) 0.0)
        (Variables|顿帧|SetHitStopActor (Variables|中间变量|GetMiddleActor))
        (bind _returnvalue_2 (Utilities|Time|SetTimerbyEvent (EventDispatchers|CreateEvent :!event EndHitStop) (Variables|中间变量|GetMiddleFloat)))
        (Variables|Default|SetTimerHandler _returnvalue_2)))))

(event EventEndHitStop
  ;[0.15 0.15 0.15 0.5 36] 接口事件
  (Variables|顿帧|SetbInHitStop false)
  (Utilities|Time|ClearandInvalidateTimerbyHandle (Variables|Default|GetTimerHandler))
  (Variables|/Script/Engine.Actor|SetCustomTimeDilation (Variables|Default|GetOwner) 1.0)
  (Variables|/Script/Engine.Actor|SetCustomTimeDilation (Variables|顿帧|GetHitStopActor) 1.0)
  (Variables|顿帧|SetHitStopAttacker 0)
  (Variables|顿帧|SetHitStopDefender 0)
  (Utilities|Time|SetGlobalTimeDilation 1.0))

(event EventPlayEnemySlowMo
  (params (Scale :type Float%20%28double-precision%29) (Duration :type Float%20%28double-precision%29))
  ;[0.15 0.15 0.15 0.5 36] 接口事件
  (Variables|放缓|SetSlowMoScale Scale)
  (Variables|放缓|SetSlowMoDuration Duration)
  (Utilities|FlowControl|Sequence
    (:then_1
      (if (Utilities|Array|IsNotEmpty (Variables|放缓|GetSlowMoActors))
        (CallFunction|RestoreSlowMo)))
    (:then_2
      (Utilities|Time|ClearandInvalidateTimerbyHandle (Variables|放缓|GetSlowMoTimerHandle))
      (bind _outactors (Actor|GetAllActorsOfClass "/Game/Enemy/BP_EnemyBase.BP_EnemyBase_C"))
      (for _array_element _outactors
        (Utilities|IsValid _array_element
          (:Is%20Valid
            (Variables|/Script/Engine.Actor|SetCustomTimeDilation _array_element (Variables|放缓|GetSlowMoScale))
            (Utilities|Array|Add (Variables|放缓|GetSlowMoActors) _array_element)))))
    (:then_3
      (bind _returnvalue (Utilities|Time|SetTimerbyEvent (EventDispatchers|CreateEvent :!event Custom|RestoreSlowMo) (Variables|放缓|GetSlowMoDuration)))
      (Variables|放缓|SetSlowMoTimerHandle _returnvalue))))

(event EventPlayPerfectBlockSound
  ;[0.15 0.15 0.15 0.5 36] 接口事件
  (bind _returnvalue (Audio|SpawnSound2D (Variables|音效|GetPerfectBlockSound) 1.0 1.0 0.0 0))
  (bind _output_get (Variables|Default|SetAudioComponent _returnvalue))
  (Audio|Parameter|SetFloatParameter _output_get "Duration" (Variables|放缓|GetSlowMoDuration) :!class /Script/Engine.AudioComponent)
  (Audio|Parameter|SetFloatParameter (Variables|Default|GetAudioComponent) "Depth" 1.5 :!class /Script/Engine.AudioComponent))

(event EventPlayPerfectDodgeStartSound
  ;[0.15 0.15 0.15 0.5 36] 接口事件
  (Utilities|Time|ClearandInvalidateTimerbyHandle (Variables|Default|GetPerfectDodgeSoundTimer))
  (bind _returnvalue (Audio|SpawnSound2D (Variables|音效|GetPerfectDodgeStartSound) 1.0 1.0 0.0 0))
  (bind _output_get (Variables|Default|SetAudioComponent _returnvalue))
  (Audio|Parameter|SetFloatParameter _output_get "Duration" (Variables|放缓|GetSlowMoDuration) :!class /Script/Engine.AudioComponent)
  (Audio|Parameter|SetFloatParameter (Variables|Default|GetAudioComponent) "Depth" 1.5 :!class /Script/Engine.AudioComponent)
  (bind _returnvalue_2 (Utilities|Time|SetTimerbyEvent (EventDispatchers|CreateEvent :!event Custom|PlayPerfectDodgeEndSound) (Variables|放缓|GetSlowMoDuration)))
  (Variables|Default|SetPerfectDodgeSoundTimer _returnvalue_2))

(event EventPlayKnockdownSound
  ;[0.15 0.15 0.15 0.5 36] 接口事件
  (Utilities|IsValid (Variables|音效|GetKnockdownImpactSound)
    (:Is%20Valid
      (Audio|PlaySoundatLocation (Variables|音效|GetKnockdownImpactSound) (Transformation|GetActorLocation (Variables|Default|GetOwner)) "0, 0, 0" 1e+01 1.0 0.0 0 0 0 0))))

(event EventPlayGrabImpactSound
  ;[0.15 0.15 0.15 0.5 36] 接口事件
  (Utilities|IsValid (Variables|音效|GetGrabImpactSound)
    (:Is%20Valid
      (Audio|PlaySoundatLocation (Variables|音效|GetGrabImpactSound) (Transformation|GetActorLocation (Variables|Default|GetOwner)) "0, 0, 0" 1e+01 1.0 0.0 0 0 0 0))))