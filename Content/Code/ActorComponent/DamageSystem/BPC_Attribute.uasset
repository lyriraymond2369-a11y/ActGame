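; BPC_Attribute is an actor component in the damage system that holds combat stats: health, poise, attack, defense and poise attack.
; HP and poise start at maximum, and getters expose stats, with attack combining weapon bonus and buff rate.
; TakeDamage clamps both pools, returning true and refilling poise when it breaks; IsDead checks HP.
; AddBonus permanently adds to base attack, while guard and poise-restore events are empty stubs.
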(event EventBeginPlay
  (Variables|Default|SetHP (Variables|Default|GetMaxHP))
  (Variables|Default|SetPoise (Variables|Default|GetMaxPoise)))

(event EventTick
  (params (DeltaSeconds :type Float%20%28single-precision%29)))

(event EventAddBonus
  (params (AttackDelta :type Float%20%28double-precision%29))
  ;[0.15 0.15 0.15 0.5] 接口事件
  (Variables|Default|SetAttack (+ AttackDelta (Variables|Default|GetAttack))))

(event EventRestorePoise
  ;[0.15 0.15 0.15 0.5] 接口事件
)

(event EventExitGuard
  ;[0.15 0.15 0.15 0.5] 接口事件
)

(event EventEnterGuard
  ;[0.15 0.15 0.15 0.5] 接口事件
)

(fn GetAttack
  (return (* (+ (Variables|Default|GetAttack) (Variables|Default|GetWeaponBonus)) (+ (Variables|Default|GetBuffBonusRate) 1.0))))

(fn GetDefense
  (return (Variables|Default|GetDefense)))

(fn GetPoiseAttack
  (return (Variables|Default|GetPoiseAttack)))

(fn IsDead
  (return (<= (Variables|Default|GetHP) 0.0)))

(fn TakeDamage
  (params (FinalDamage :type Float%20%28double-precision%29) (PoiseDamage :type Float%20%28double-precision%29))
  (Utilities|FlowControl|Sequence
    (:then_0
      (Variables|Default|SetHP (Math|Float|Clamp(Float) (- (Variables|Default|GetHP) FinalDamage) 0.0 (Variables|Default|GetMaxHP))))
    (:then_1
      (bind _output_get (Variables|Default|SetPoise (Math|Float|Clamp(Float) (- (Variables|Default|GetPoise) PoiseDamage) 0.0 (Variables|Default|GetMaxPoise))))
      (if (<= _output_get 0.0)
        (Variables|Default|SetPoise (Variables|Default|GetMaxPoise))
        (return true)
        (else
          (return false))))))