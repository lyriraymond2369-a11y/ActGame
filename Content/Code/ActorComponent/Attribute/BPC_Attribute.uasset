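; Actor component holding combat attributes (HP, poise, attack, defense, team) and resolving incoming hits.
; ReceiveDamage checks death, invincibility with timed perfect dodge, then frontal guard; the perfect-block branch is hard-wired off.
; TakeDamage applies HP and poise loss, refilling poise on break, while dispatchers report dodges and applied hits.
; Ending a dodge grants a timer-based invincibility tail; unguarded damage uses the component's own Attack, not incoming BaseDamage.
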(event Custom|GrantPerfectDodgeTail
  ;[0.15 0.15 0.15 0.5 36] 中间事件
  (Variables|Default|SetbInvincibleTail true)
  (Utilities|Time|ClearandInvalidateTimerbyHandle (Variables|Default|GetTailTimerHandle))
  (bind _returnvalue (Utilities|Time|SetTimerbyEvent (delegate Custom|ClearInvincibleTail) (Variables|闪避|GetPerfectDodgeTailDuration)))
  (Variables|Default|SetTailTimerHandle _returnvalue))

(event Custom|ClearInvincibleTail
  ;[0.15 0.15 0.15 0.5 36] 中间事件
  (Variables|Default|SetbInvincibleTail false))

(event Custom|ClearDodgeState
  ;[0.15 0.15 0.15 0.5 36] 中间事件
  (if (not (Variables|Default|GetbPerfectDodgeUsed))
    (Variables|Default|SetbPerfectDodgeUsed true)))

(event EventBeginPlay
  (Variables|属性|SetHP (Variables|属性|GetMaxHP))
  (Variables|属性|SetPoise (Variables|属性|GetMaxPoise))
  (Variables|Default|SetOwner (Components|GetOwner)))

(event EventTick
  (params (DeltaSeconds :type Float%20%28single-precision%29)))

(event EventAddBonus
  (params (AttackDelta :type Float%20%28double-precision%29))
  ;[0.15 0.15 0.15 0.5] 接口事件
  (Variables|属性|SetWeaponBonus AttackDelta))

(event EventRestorePoise
  ;[0.15 0.15 0.15 0.5] 接口事件
)

(event EventExitGuard
  ;[0.15 0.15 0.15 0.5] 接口事件
  (Variables|格挡|SetbIsGuarding false))

(event EventEnterGuard
  ;[0.15 0.15 0.15 0.5] 接口事件
  (Variables|格挡|SetbIsGuarding true)
  (Variables|格挡|SetLastGuardTime (Utilities|Time|GetGameTimeinSeconds))
  (Variables|格挡|SetbPerfectBlockUsed false))

(event EventClearPoseBroken
  ;[0.15 0.15 0.15 0.5] 接口事件
)

(event EventNotifyDodgeStart
  (params (Time :type Float%20%28double-precision%29))
  ;[0.15 0.15 0.15 0.5] 接口事件
  (Variables|闪避|SetLastDodgeTime Time)
  (Variables|Default|SetbPerfectDodgeUsed false))

(event EventSetInvincible
  (params (Val :type Boolean))
  ;[0.15 0.15 0.15 0.5] 接口事件
  (Variables|Default|SetbInvincible Val))

(event EventEndPerfectDodge
  ;[0.15 0.15 0.15 0.5] 接口事件
  (if (Variables|Default|GetbInvincible)
    (CallFunction|SetInvincible false)
    (CallFunction|GrantPerfectDodgeTail)))

(fn IsPerfect?
  (params (LastTime :type Float%20%28double-precision%29) (WindowTime :type Float%20%28double-precision%29))
  (return (<= (|((a-b)-c) (Utilities|Time|GetGameTimeinSeconds) LastTime WindowTime) 0.0)))

(fn IsAttackFront?
  (params (HitPoint :type Vector))
  (return (>= (Math|Vector|DotProduct (- HitPoint (Transformation|GetActorLocation (Variables|Default|GetOwner))) (Transformation|GetActorForwardVector (Variables|Default|GetOwner))) (Variables|Default|GetFrontDotThreshold))))

(fn GetHitDirection
  (params (HitLoc :type Vector))
  (LocalVariables|SetHitPoint HitLoc)
  (LocalVariables|SetToAttack (Math|Vector|Normalize (- (LocalVariables|GetHitPoint) (Transformation|GetActorLocation (Variables|Default|GetOwner)))))
  (LocalVariables|SetDot (Math|Vector|DotProduct (Transformation|GetActorForwardVector (Variables|Default|GetOwner)) (LocalVariables|GetToAttack)))
  (LocalVariables|SetSide (Math|Vector|DotProduct (Transformation|GetActorRightVector (Variables|Default|GetOwner)) (LocalVariables|GetToAttack)))
  (Utilities|FlowControl|Sequence
    (:then_0
      (if (>= (LocalVariables|GetDot) (Math|Trig|Cos(Degrees) 45.0))
        (return "NewEnumerator0")))
    (:then_1
      (if (<= (LocalVariables|GetDot) (Math|Trig|Cos(Degrees) 135.0))
        (return "NewEnumerator1")))
    (:then_2
      (if (>= (LocalVariables|GetSide) 0.0)
        (return "NewEnumerator3")))
    (:then_3
      (return "NewEnumerator2"))))

(fn IsInvincible
  (return (or (Variables|Default|GetbInvincible) (Variables|Default|GetbInvincibleTail))))

(fn GetAttack
  (return (* (+ (Variables|属性|GetAttack) (Variables|属性|GetWeaponBonus)) (+ (Variables|属性|GetBuffBonusRate) 1.0))))

(fn GetDefense
  (return (Variables|属性|GetDefense)))

(fn GetPoiseAttack
  (return (Variables|属性|GetPoiseAttack)))

(fn GetTeam
  (return (Variables|属性|GetTeam)))

(fn IsDead
  (return (<= (Variables|属性|GetHP) 0.0)))

(fn ReceiveDamage
  (params (ATK :type ST%20Attack%20Data%20Structure) (BaseDamage :type Float%20%28double-precision%29) (BasePoiseDamage :type Float%20%28double-precision%29) (HitLocation :type Vector :default "0, 0, 0") (HitPoint :type Vector :default "0, 0, 0"))
  (LocalVariables|SetAttackData ATK)
  (LocalVariables|SetAttackHP BaseDamage)
  (LocalVariables|SetAttackPoise BasePoiseDamage)
  (LocalVariables|SetHitActorLocation HitLocation)
  (LocalVariables|SetHitPointLocation HitPoint)
  (Utilities|FlowControl|Sequence
    (:then_0
      (bind _hitdirection (CallFunction|GetHitDirection (LocalVariables|GetHitActorLocation)))
      (LocalVariables|SetHitDirection _hitdirection))
    (:then_1
      (bind _rezult (CallFunction|IsAttackFront? (LocalVariables|GetHitActorLocation)))
      (LocalVariables|SetbFront _rezult))
    (:then_2
      (bind _dead (CallFunction|IsDead))
      (if _dead
        (return "NewEnumerator0" false false false)))
    (:then_3
      (bind _rezult_2 (CallFunction|IsInvincible))
      (if _rezult_2
        (bind _rezult_3 (CallFunction|IsPerfect? (Variables|闪避|GetLastDodgeTime) (Variables|闪避|GetPerfectDodgeWindow)))
        (if (and _rezult_3 (Variables|Default|GetbInvincible))
          (CallFunction|ClearDodgeState)
          (Default|CallOnPerfectDodge)
          (return "NewEnumerator0" false false true)
          (else
            (return "NewEnumerator0" false false false)))))
    (:then_4
      (bind _rezult_4 (CallFunction|IsPerfect? (Variables|格挡|GetLastGuardTime) (Variables|格挡|GetPerfectGuardWindow)))
      (if (Math|Boolean|ANDBoolean _rezult_4 false (Variables|格挡|GetbIsGuarding) (LocalVariables|GetbFront))
        (if (not (Variables|格挡|GetbPerfectBlockUsed))
          (Variables|格挡|SetbPerfectBlockUsed true)
          (Default|CallOnPerfectBlock (LocalVariables|GetHitPointLocation))
          (return "NewEnumerator2" true false false))))
    (:then_5
      (if (Math|Boolean|ANDBoolean (Variables|格挡|GetbIsGuarding) (LocalVariables|GetbFront) true)
        (LocalVariables|SetFinalDamage (|(((a*b)*(1-c))*d) (LocalVariables|GetAttackHP) (.DamageRate (Utilities|Struct|BreakST_AttackData (LocalVariables|GetAttackData))) (Variables|属性|GetDefense) (Variables|格挡|GetGuardDamageRate)))
        (LocalVariables|SetFinalPoiseDamage (|((a*b)*c) (LocalVariables|GetAttackPoise) (.PoiseDdamageRate (Utilities|Struct|BreakST_AttackData (LocalVariables|GetAttackData))) (Variables|格挡|GetGuardPoiseRate)))
        (bind _rezult_5 (CallFunction|TakeDamage (LocalVariables|GetFinalDamage) (LocalVariables|GetFinalPoiseDamage)))
        (bind _output_get (LocalVariables|SetMiddleBool _rezult_5))
        (if _output_get
          (Default|CallOnDamageApplied "NewEnumerator1" (LocalVariables|GetHitDirection) (LocalVariables|GetMiddleBool))
          (return "NewEnumerator1" false (LocalVariables|GetMiddleBool) false)
          (else
            (Default|CallOnDamageApplied "NewEnumerator2" (LocalVariables|GetHitDirection) (LocalVariables|GetMiddleBool))
            (return "NewEnumerator2" false (LocalVariables|GetMiddleBool) false)))))
    (:then_6
      (LocalVariables|SetFinalDamage (|((a*b)*(1-c)) (.DamageRate (Utilities|Struct|BreakST_AttackData (LocalVariables|GetAttackData))) (Variables|属性|GetAttack) (Variables|属性|GetDefense)))
      (LocalVariables|SetFinalPoiseDamage (|(a*b) (.PoiseDdamageRate (Utilities|Struct|BreakST_AttackData (LocalVariables|GetAttackData))) (LocalVariables|GetAttackPoise)))
      (bind _rezult_6 (CallFunction|TakeDamage (LocalVariables|GetFinalDamage) (LocalVariables|GetFinalPoiseDamage)))
      (LocalVariables|SetMiddleBool _rezult_6)
      (Default|CallOnDamageApplied "NewEnumerator1" (LocalVariables|GetHitDirection) (LocalVariables|GetMiddleBool))
      (return "NewEnumerator1" false (LocalVariables|GetMiddleBool) false))))

(fn TakeDamage
  (params (FinalDamage :type Float%20%28double-precision%29) (PoiseDamage :type Float%20%28double-precision%29))
  (Utilities|FlowControl|Sequence
    (:then_0
      (Variables|属性|SetHP (Math|Float|Clamp(Float) (- (Variables|属性|GetHP) FinalDamage) 0.0 (Variables|属性|GetMaxHP))))
    (:then_1
      (bind _output_get (Variables|属性|SetPoise (Math|Float|Clamp(Float) (- (Variables|属性|GetPoise) PoiseDamage) 0.0 (Variables|属性|GetMaxPoise))))
      (if (<= _output_get 0.0)
        (Variables|属性|SetPoise (Variables|属性|GetMaxPoise))
        (return true)
        (else
          (return false))))))