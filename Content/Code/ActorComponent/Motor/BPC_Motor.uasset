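; BPC_Motor is an actor component that drives a Character's movement for knockbacks, gravity changes and montage movement.
; Knockback stops movement, then applies velocity-change impulses, boosting the horizontal part.
; A motion profile sets an actor-relative direction; starting motion applies its vertical kick and, for fast profiles, temporarily overrides speed, friction, gravity and rotation.
; Tick feeds scaled movement input until stopped or a safety timeout restores the saved settings.
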(event Custom|UpdateMontageMove
  ;[0.15 0.15 0.15 0.5 36] 中间事件
  (if (Variables|Default|GetbMotionActive)
    (if (>= (Variables|/Script/Engine.CharacterMovementComponent|GetMaxWalkSpeed (Variables|Default|GetCharacter%20Movement)) (Variables|Default|GetMotionSpeedThreshold))
      (if (>= (Utilities|Time|GetGameTimeinSeconds) (Variables|Default|GetMotionSafetyEndTime))
        (CallFunction|StopMotion)
        (else
          (Pawn|Input|AddMovementInput (Variables|Default|GetOwnerCharacter) (Variables|Default|GetMotionDirection) (Variables|Default|GetMotionScale) false))))))

(event EventBeginPlay
  (bind _output_get (Variables|Default|SetOwner (Components|GetOwner)))
  (bind _charactermovement (Class|BPICharacterBase|GetCharacterMovement(Message) _output_get))
  (Variables|Default|SetCharacter%20Movement _charactermovement)
  (bind _as角色 (Utilities|Casting|CastToCharacter (Variables|Default|GetOwner)))
  (Variables|Default|SetOwnerCharacter _as角色))

(event EventTick
  (params (DeltaSeconds :type Float%20%28single-precision%29))
  (CallFunction|UpdateMontageMove))

(event EventApplyKnockback
  (params (Force :type Vector :default "0, 0, 0") (bIgnoreMove :type Boolean))
  ;[0.15 0.15 0.15 0.5] 接口方法
  (Variables|中间变量|SetMiddleVector3 Force)
  (Variables|中间变量|SetMiddleBool bIgnoreMove)
  (Variables|Default|GetOwner
    (:then
      (Utilities|FlowControl|Sequence
        (:then_0
          (Components|Movement|StopMovementImmediately (Variables|Default|GetCharacter%20Movement))
          (Physics|AddImpulse (Variables|Default|GetCharacter%20Movement) (* (CallFunction|GetXYImpluse (Variables|中间变量|GetMiddleVector3)) 3.0) true)
          (Physics|AddImpulse (Variables|Default|GetCharacter%20Movement) (Math|Vector|MakeVector 0.0 0.0 (.Z (Math|Vector|BreakVector (Variables|中间变量|GetMiddleVector3)))) true))))
    (:else)))

(event EventSetMotionProfile
  (params (profile :type ST%20Motion%20Profile%20Structure))
  ;[0.15 0.15 0.15 0.5] 接口方法
  (bind _output_get (Variables|Default|SetMotionProfile profile))
  (Variables|Default|SetMotionDirection (CallFunction|GetDirection (.direction (Utilities|Struct|BreakST_MotionProfile _output_get))))
  (Variables|Default|SetZMotion (Math|Vector|MakeVector 0.0 0.0 (.Z (Math|Vector|BreakVector (.direction (Utilities|Struct|BreakST_MotionProfile _output_get)))))))

(event EventStartMotion
  (bind _motionprofile (Variables|Default|GetMotionProfile))
  (bind (_speed _direction _friction _gravityscale) (Utilities|Struct|BreakST_MotionProfile _motionprofile))
  ;[0.15 0.15 0.15 0.5] 接口方法
  (if (not (Variables|Default|GetbMotionActive))
    (CallFunction|ApplyKnockback (Variables|Default|GetZMotion) false)
    (if (>= (.speed (Utilities|Struct|BreakST_MotionProfile (Variables|Default|GetMotionProfile))) 6.1e+02)
      (Utilities|FlowControl|Sequence
        (:then_0
          (Variables|/Script/Engine.CharacterMovementComponent|SetMaxAcceleration (Variables|Default|GetCharacter%20Movement) 3.6e+04)
          (Variables|Original|SetOriginalMaxSpeed (Variables|/Script/Engine.CharacterMovementComponent|GetMaxWalkSpeed (Variables|Default|GetCharacter%20Movement)))
          (Variables|Original|SetOriginalOrientRotation true)
          (Variables|Original|SetOriginalGravityScale (Variables|/Script/Engine.CharacterMovementComponent|GetGravityScale (Variables|Default|GetCharacter%20Movement)))
          (Variables|Original|SetOriginalBraking (Variables|/Script/Engine.CharacterMovementComponent|GetGroundFriction (Variables|Default|GetCharacter%20Movement))))
        (:then_1
          (Variables|/Script/Engine.CharacterMovementComponent|SetMaxWalkSpeed (Variables|Default|GetCharacter%20Movement) _speed)
          (Variables|/Script/Engine.CharacterMovementComponent|SetbOrientRotationToMovement (Variables|Default|GetCharacter%20Movement) false)
          (Variables|/Script/Engine.CharacterMovementComponent|SetGroundFriction (Variables|Default|GetCharacter%20Movement) _friction)
          (Variables|/Script/Engine.CharacterMovementComponent|SetGravityScale (Variables|Default|GetCharacter%20Movement) _gravityscale)
          (Variables|Default|SetbMotionActive true)
          (Variables|Default|SetMotionSafetyEndTime (+ (Utilities|Time|GetGameTimeinSeconds) 1.2)))))))

(event EventStopMotion
  ;[0.15 0.15 0.15 0.5] 接口方法
  (if (Variables|Default|GetbMotionActive)
    (Variables|Default|SetbMotionActive false)
    (Utilities|FlowControl|Sequence
      (:then_1
        (Variables|/Script/Engine.CharacterMovementComponent|SetMaxWalkSpeed (Variables|Default|GetCharacter%20Movement) (Variables|Original|GetOriginalMaxSpeed))
        (Variables|/Script/Engine.CharacterMovementComponent|SetbOrientRotationToMovement (Variables|Default|GetCharacter%20Movement) (Variables|Original|GetOriginalOrientRotation))
        (Variables|/Script/Engine.CharacterMovementComponent|SetGroundFriction (Variables|Default|GetCharacter%20Movement) (Variables|Original|GetOriginalBraking))
        (Variables|/Script/Engine.CharacterMovementComponent|SetGravityScale (Variables|Default|GetCharacter%20Movement) (Variables|Original|GetOriginalGravityScale))))))

(event EventSetGravity
  (params (Scale :type Float%20%28double-precision%29))
  ;[0.15 0.15 0.15 0.5] 接口方法
  (Variables|/Script/Engine.CharacterMovementComponent|SetGravityScale (Variables|Default|GetCharacter%20Movement) Scale))

(event EventResetGravity
  ;[0.15 0.15 0.15 0.5] 接口方法
  (Variables|/Script/Engine.CharacterMovementComponent|SetGravityScale (Variables|Default|GetCharacter%20Movement) 1.0))

(event EventSetMotionScale
  (params (Rate :type Float%20%28double-precision%29))
  ;[0.15 0.15 0.15 0.5] 接口方法
  (Variables|Default|SetMotionScale Rate))

(fn GetDirection
  (params (Original :type Vector))
  (bind (_x _y) (Math|Vector|BreakVector Original))
  (return (Math|Vector|Normalize (+ (* (Transformation|GetActorForwardVector (Variables|Default|GetOwner)) _x) (* _y (Transformation|GetActorRightVector (Variables|Default|GetOwner)))))))

(fn GetXYImpluse
  (params (Val :type Vector))
  (bind (_x _y) (Math|Vector|BreakVector Val))
  (return (Math|Vector|MakeVector _x _y 0.0)))

(fn IsMoving
  (return false))