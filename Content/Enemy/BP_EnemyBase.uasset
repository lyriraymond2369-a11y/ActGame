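; Base enemy character that hosts attribute, motor, attack trace and combat feedback components for combat.
; On BeginPlay it spawns a BP_Player_Sword on the right-hand socket, copies its bonus into the attribute component and caches its hitbox.
; Message-style getters expose these parts, plus the AI component held on its AIC_EnemyBase controller.
; It also answers death and team-based hostility queries and takes impulses through LaunchCharacter.
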(event Custom|InitWeapon
  ;[0.15 0.15 0.15 0.5] 初始化
  (bind _returnvalue (Game|SpawnActorfromClass "/Game/Code/Weapon/BP_Player_Sword.BP_Player_Sword_C" (Math|Transform|MakeTransform "0, 0, 0" "0, 0, 0" "1.000000,1.000000,1.000000") "Undefined" "MultiplyWithRoot" 0 5.0 0))
  (bind _output_get (Variables|Default|SetWeapon _returnvalue))
  (Transformation|AttachComponentToComponent _output_get (Variables|Character|GetMesh) "Weapon_R" "KeepRelative" "KeepRelative" "KeepRelative" true)
  (CallFunction|FixedUpdateAttributeComponent)
  (bind _hitbox (Class|BPIWeaponBase|GetWeaponHitBox(Message) (Variables|Default|GetWeapon)))
  (Variables|Default|SetHit%20Box _hitbox))

(event Custom|FixedUpdateAttributeComponent
  (bind _weapon (Variables|Default|GetWeapon))
  ;[0.15 0.15 0.15 0.5 36] 修改时更新
  (bind _weaponbonus (Class|BPIWeaponBase|GetWeaponBonus(Message) _weapon))
  (Variables|/Game/Code/ActorComponent/Attribute/BPC_Attribute.BPC_Attribute_C|SetWeaponBonus (Variables|Default|GetBPC_Attribute) (select (Utilities|IsValid _weapon) _weaponbonus 0.0)))

(event EventBeginPlay
  (CallFunction|InitWeapon))

(event Collision|EventActorBeginOverlap
  (params (OtherActor :type Actor%20Object%20Reference)))

(event EventTick
  (params (DeltaSeconds :type Float%20%28single-precision%29)))

(event EventApplyImpulse
  (params (Vector :type Vector :default "0, 0, 0") (XYOverride :type Boolean) (ZOverride :type Boolean))
  ;[0.15 0.15 0.15 0.5 36] 接口事件
  (Character|LaunchCharacter Vector XYOverride ZOverride))

(fn ConstructionScript)

(fn GetAIComponent
  (bind _asaic_enemy_base (Utilities|Casting|CastToAIC_EnemyBase (AI|GetAIController self)))
  (return (Variables|/Game/Enemy/AI/AIC_EnemyBase.AIC_EnemyBase_C|GetBPC_AI _asaic_enemy_base)))

(fn GetAttackTraceComponent
  (return (Variables|Default|GetBPC_AttackTrace)))

(fn GetAttributeComponent
  (return (Variables|Default|GetBPC_Attribute)))

(fn GetCharacterMovement
  (return (Variables|Character|GetCharacterMovement)))

(fn GetCombatFeedbackComponent
  (return (Variables|Default|GetBPC_CombatFeedBack)))

(fn GetHitBoxComponent
  (return (Variables|Default|GetHit%20Box)))

(fn GetMeshComponent
  (return (Variables|Character|GetMesh)))

(fn GetMotorComponent
  (return (Variables|Default|GetBPC_Motor)))

(fn GetWeapon
  (return (Variables|Default|GetWeapon)))

(fn IsCharacterDead
  (bind _dead (Class|BPIAttribute|IsDead(Message) (Variables|Default|GetBPC_Attribute)))
  (return _dead))

(fn IsHostile
  (params (Other :type Actor%20Object%20Reference))
  (bind _attribute (Class|BPICharacterBase|GetAttributeComponent(Message) Other))
  (bind _team (Class|BPIAttribute|GetTeam(Message) _attribute))
  (bind _team_2 (Class|BPIAttribute|GetTeam(Message) (Variables|Default|GetBPC_Attribute)))
  (return (Utilities|Enum|NotEqual(Enum) _team_2 _team)))