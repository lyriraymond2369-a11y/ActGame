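; Enemy AI component on an AIController that owns combat state and mirrors it, with target and distance, to the Blackboard.
; Each tick it prunes sight-fed perceived actors and targets the nearest hostile in range.
; Damage triggers priority-checked hit or knockdown states and releases the pawn's GameState token, which gates attacking.
; Hit stamps flag pending reactions until consumed through the AI interface, which also exposes state changes and queries.
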(event Custom|Init
  ;[0.15 0.15 0.15 0.5 36] 中间事件
  (bind _asai控制器 (Utilities|Casting|CastToAIController (Components|GetOwner)))
  (Variables|Default|SetAIOwner _asai控制器)
  (bind _as角色 (Utilities|Casting|CastToCharacter (Pawn|GetControlledPawn (Variables|Default|GetAIOwner))))
  (bind _output_get (Variables|Default|SetPawnRef _as角色))
  (bind _attribute (Class|BPICharacterBase|GetAttributeComponent(Message) _output_get))
  (Variables|Default|SetAttributeRef _attribute)
  (Variables|Default|SetCurrentState "NewEnumerator0")
  (Variables|Default|SetBlackBoard (Variables|/Script/AIModule.AIController|GetBlackboard (Variables|Default|GetAIOwner))))

(event Custom|UpdatePerception
  ;[0.15 0.15 0.15 0.5 36] 更新
  (Utilities|Array|Clear (Variables|Default|GetBadActors))
  (Utilities|FlowControl|Sequence
    (:then_0
      (for _array_element (Variables|Default|GetPerceivedActors)
        (Variables|中间变量|SetUpdateActor _array_element)
        (Utilities|FlowControl|Sequence
          (:then_0
            (Utilities|IsValid (Variables|中间变量|GetUpdateActor)
              (:Is%20Not%20Valid
                (Utilities|Array|AddUnique (Variables|Default|GetBadActors) (Variables|中间变量|GetUpdateActor)))))
          (:then_1
            (if (== (Variables|中间变量|GetUpdateActor) (Variables|Default|GetPawnRef))
              (Utilities|Array|AddUnique (Variables|Default|GetBadActors) (Variables|中间变量|GetUpdateActor))))
          (:then_2
            (bind _rezult (Class|BPICharacterBase|IsCharacterDead(Message) (Variables|中间变量|GetUpdateActor)))
            (if _rezult
              (Utilities|Array|AddUnique (Variables|Default|GetBadActors) (Variables|中间变量|GetUpdateActor))))
          (:then_3
            (bind _rezult_2 (Class|BPICharacterBase|IsHostile(Message) (Variables|Default|GetPawnRef) (Variables|中间变量|GetUpdateActor)))
            (if (not _rezult_2)
              (Utilities|Array|AddUnique (Variables|Default|GetBadActors) (Variables|中间变量|GetUpdateActor)))))))
    (:then_1
      (for _array_element_2 (Variables|Default|GetBadActors)
        (Utilities|Array|RemoveItem (Variables|Default|GetPerceivedActors) _array_element_2)))))

(event Custom|HandleKnockdown
  (params (HitDirection :type E_HitDirection%20Enum :default "NewEnumerator0"))
  ;[0.15 0.15 0.15 0.5 36] 中间事件
  (CallFunction|ApplyState "NewEnumerator12"))

(event Custom|ApplyState
  (params (New :type E_AIState%20Enum :default "NewEnumerator0"))
  ;[0.15 0.15 0.15 0.5 36] 中间事件
  (Variables|Default|SetCurrentState New)
  (CallFunction|SyncBlackboard)
  (if (Utilities|Enum|Equal(Enum) (Variables|Default|GetCurrentState) "NewEnumerator8")
    (Components|Movement|StopMovementImmediately (Variables|Default|GetCharacter%20Movement))))

(event Custom|HandleDamageApplied
  (params (HitOutCome :type E_HitOutCome%20Enum :default "NewEnumerator0") (HitDirection :type E_HitDirection%20Enum :default "NewEnumerator0") (bPoiseBroken :type Boolean))
  (Variables|中间变量|SetMiddleHitOutCome HitOutCome)
  (Variables|中间变量|SetMiddleHitDirection HitDirection)
  (Variables|中间变量|SetMiddleBool bPoiseBroken)
  (bind _alive (CallFunction|AIIsAlive))
  (if _alive
    (switch Utilities|FlowControl|Switch|SwitchonE_HitOutCome (Variables|中间变量|GetMiddleHitOutCome)
      (:NewEnumerator1
        (bind _rezult (CallFunction|AITryEnterState (select (Variables|中间变量|GetMiddleBool) "NewEnumerator11" "NewEnumerator10")))
        (if _rezult
          (Math|Integer|IncrementInt (Variables|Default|GetHitStamp)
            (:%20%20
              (CallFunction|SyncBlackboard)
              (AI|Components|Blackboard|SetValueasEnum (Variables|Default|GetBlackBoard) (Variables|KeyName|GetHitDirectionKeyName) (Variables|中间变量|GetMiddleHitDirection))
              (CallFunction|ReleaseToken)))))
      (:NewEnumerator6
        (bind _rezult_2 (CallFunction|AITryEnterState "NewEnumerator12"))
        (if _rezult_2
          (CallFunction|HandleKnockdown (Variables|中间变量|GetMiddleHitDirection))
          (Class|BPIGameState|RemoveToken(Message) (Game|GetGameState) (Variables|Default|GetPawnRef)))))))

(event Custom|SyncBlackboard
  ;[0.15 0.15 0.15 0.5 36] 中间事件
  (AI|Components|Blackboard|SetValueasEnum (Variables|Default|GetBlackBoard) (Variables|KeyName|GetAIStateKeyName) (Variables|Default|GetCurrentState))
  (AI|Components|Blackboard|SetValueasBool (Variables|Default|GetBlackBoard) (Variables|KeyName|GetIsControlledKeyName) (CallFunction|IsControlled (Variables|Default|GetCurrentState)))
  (AI|Components|Blackboard|SetValueasBool (Variables|Default|GetBlackBoard) (Variables|KeyName|GetHitPendingKeyName) (> (Variables|Default|GetHitStamp) (Variables|Default|GetHandledStamp))))

(event Custom|UpdateDistances
  ;[0.15 0.15 0.15 0.5 36] 更新
  (Utilities|IsValid (Variables|Default|GetTarget)
    (:Is%20Valid
      (bind _output_get (Variables|Default|SetDisToTarget (Math|Vector|Distance(Vector) (Transformation|GetActorLocation (Variables|Default|GetPawnRef)) (Transformation|GetActorLocation (Variables|Default|GetTarget)))))
      (AI|Components|Blackboard|SetValueasFloat (Variables|Default|GetBlackBoard) (Variables|KeyName|GetDisToTargetKeyName) _output_get))
    (:Is%20Not%20Valid
      (bind _output_get_2 (Variables|Default|SetDisToTarget -1.0))
      (AI|Components|Blackboard|SetValueasFloat (Variables|Default|GetBlackBoard) (Variables|KeyName|GetDisToTargetKeyName) _output_get_2))))

(event Custom|UpdateRefreshTarget
  ;[0.15 0.15 0.15 0.5 36] 更新
  (bind _actor (CallFunction|PickTarget))
  (bind _output_get (Variables|Default|SetTarget _actor))
  (AI|Components|Blackboard|SetValueasObject (Variables|Default|GetBlackBoard) (Variables|KeyName|GetTargetKeyName) _output_get))

(event Custom|AddPerceivedActor
  (params (Perceived :type Actor%20Object%20Reference))
  ;[0.15 0.15 0.15 0.5 36] 中间事件
  (Utilities|IsValid Perceived
    (:Is%20Valid
      (Utilities|Array|AddUnique (Variables|Default|GetPerceivedActors) Perceived))))

(event Custom|RemovePerceivedActor
  (params (Perceived :type Actor%20Object%20Reference))
  ;[0.15 0.15 0.15 0.5 36] 中间事件
  (Utilities|Array|RemoveItem (Variables|Default|GetPerceivedActors) Perceived))

(event EventBeginPlay
  (CallFunction|Init)
  (EventDispatchers|BindEventtoOnDamageApplied (Variables|Default|GetAttributeRef) (delegate Custom|HandleDamageApplied))
  (bind _charactermovement (Class|BPICharacterBase|GetCharacterMovement(Message) (Variables|Default|GetPawnRef)))
  (Variables|Default|SetCharacter%20Movement _charactermovement))

(event EventTick
  (params (DeltaSeconds :type Float%20%28single-precision%29))
  (Utilities|FlowControl|Sequence
    (:then_0
      (CallFunction|UpdatePerception)
      (CallFunction|UpdateRefreshTarget)
      (CallFunction|UpdateDistances))))

(event EventAIHandleSight
  (params (Actor :type Actor%20Object%20Reference) (bSensed :type Boolean))
  ;[0.15 0.15 0.15 0.5 36] 接口事件
  (Variables|中间变量|SetMiddleActor Actor)
  (Variables|中间变量|SetMiddleBool bSensed)
  (Utilities|IsValid (Variables|中间变量|GetMiddleActor)
    (:Is%20Valid
      (Utilities|FlowControl|Sequence
        (:then_0
          (if (Variables|中间变量|GetMiddleBool)
            (bind _rezult (Class|BPICharacterBase|IsHostile(Message) (Variables|Default|GetPawnRef) (Variables|中间变量|GetMiddleActor)))
            (if _rezult
              (CallFunction|AddPerceivedActor (Variables|中间变量|GetMiddleActor)))
            (else
              (CallFunction|RemovePerceivedActor (Variables|中间变量|GetMiddleActor)))))
        (:then_1
          (CallFunction|UpdateRefreshTarget))))))

(event EventAISetState
  (params (NewState :type E_AIState%20Enum :default "NewEnumerator0"))
  ;[0.15 0.15 0.15 0.5 36] 接口事件
  (CallFunction|ApplyState NewState))

(event EventAIReturntoInitialState
  ;[0.15 0.15 0.15 0.5 36] 接口事件
  (CallFunction|ApplyState (select (Utilities|IsValid (Variables|Default|GetTarget)) "NewEnumerator7" "NewEnumerator0")))

(fn PickTarget
  (LocalVariables|SetBestDis (Variables|Default|GetCreatureSightRange))
  (for _array_element (Variables|Default|GetPerceivedActors)
    (LocalVariables|SetPerceivedActor _array_element)
    (Utilities|IsValid (LocalVariables|GetPerceivedActor)
      (:Is%20Valid
        (bind _rezult (Class|BPICharacterBase|IsHostile(Message) (Variables|Default|GetPawnRef) (LocalVariables|GetPerceivedActor)))
        (if _rezult
          (if (< (Math|Vector|Distance(Vector) (Transformation|GetActorLocation (Variables|Default|GetPawnRef)) (Transformation|GetActorLocation (LocalVariables|GetPerceivedActor))) (LocalVariables|GetBestDis))
            (LocalVariables|SetBestDis (Math|Vector|Distance(Vector) (Transformation|GetActorLocation (Variables|Default|GetPawnRef)) (Transformation|GetActorLocation (LocalVariables|GetPerceivedActor))))
            (LocalVariables|SetBest (LocalVariables|GetPerceivedActor)))))))
  (return (LocalVariables|GetBest) (LocalVariables|GetBestDis)))

(fn EvaluateTransition
  (if (and (Utilities|IsValid (Variables|Default|GetPawnRef)) (Utilities|IsValid (Variables|Default|GetAttributeRef)))
    (bind _dead (Class|BPIAttribute|IsDead(Message) (Variables|Default|GetAttributeRef)))
    (if (not _dead)
      (if (Utilities|Enum|NotEqual(Enum) (Variables|Default|GetCurrentState) "NewEnumerator8")
        (if (Utilities|IsValid 0)
          (switch Utilities|FlowControl|Switch|SwitchonE_AIState (Variables|Default|GetCurrentState)
            (:NewEnumerator0
              (if (<= (Variables|Default|GetDisToTarget) (Variables|Default|GetCreatureSightRange))
                (return "NewEnumerator7")
                (else
                  (return (Variables|Default|GetCurrentState)))))
            (:NewEnumerator7
              (if (> (Variables|Default|GetDisToTarget) (Variables|Default|GetCreatureSightRange))
                (return "NewEnumerator0")
                (else
                  (return (Variables|Default|GetCurrentState)))))
            (:NewEnumerator8
              (return "NewEnumerator8")))
          (else
            (return "NewEnumerator0")))
        (else
          (return "NewEnumerator8")))
      (else
        (return "NewEnumerator8")))
    (else
      (return (Variables|Default|GetCurrentState)))))

(fn ComputeNextState
  (Utilities|FlowControl|Sequence
    (:then_0
      (bind _rezult (Condition|DeadCondition))
      (if _rezult
        (return "NewEnumerator8")))
    (:then_1
      (bind _rezult_2 (条件|AttackCondition))
      (if _rezult_2
        (return "NewEnumerator9")))
    (:then_2
      (bind _rezult_3 (条件|IdleCondition))
      (if _rezult_3
        (return "NewEnumerator0")))
    (:then_3
      (if (Utilities|Enum|Equal(Enum) (Variables|Default|GetCurrentState) "NewEnumerator9")
        (return "NewEnumerator9")
        (else
          (return "NewEnumerator7"))))))

(fn DeadCondition
  (bind _dead (Class|BPIAttribute|IsDead(Message) (Variables|Default|GetAttributeRef)))
  (return (or (Utilities|Enum|Equal(Enum) (Variables|Default|GetCurrentState) "NewEnumerator8") _dead)))

(fn AttackCondition
  (bind _rezult (CallFunction|TryAcquireToken))
  (bind _rezult_2 (Class|BPICharacterBase|IsHostile(Message) (Variables|Default|GetPawnRef) (Variables|Default|GetTarget)))
  (return (Math|Boolean|ANDBoolean (or (Utilities|Enum|Equal(Enum) (Variables|Default|GetCurrentState) "NewEnumerator9") (and (Utilities|Enum|Equal(Enum) (Variables|Default|GetCurrentState) "NewEnumerator7") (<= (Variables|Default|GetDisToTarget) 3e+02))) _rezult _rezult_2)))

(fn IdleCondition
  (bind _rezult (Class|BPICharacterBase|IsHostile(Message) (Variables|Default|GetPawnRef) (Variables|Default|GetTarget)))
  (return (or (not (Utilities|IsValid (Variables|Default|GetPawnRef))) (not (Utilities|IsValid (Variables|Default|GetTarget))))))

(fn IsControlled
  (params (State :type E_AIState%20Enum :default "NewEnumerator0"))
  (return (Utilities|Select :Index State :NewEnumerator0 false :NewEnumerator7 false :NewEnumerator8 true :NewEnumerator9 false :NewEnumerator10 true :NewEnumerator11 true :NewEnumerator12 true)))

(fn CaninNewState
  (params (NewState :type E_AIState%20Enum :default "NewEnumerator0"))
  (bind _aistateproperty (Variables|Default|GetAIStateProperty))
  (bind _currentstate (Variables|Default|GetCurrentState))
  (bind (_value _returnvalue) (Utilities|Map|Find _aistateproperty _currentstate))
  (LocalVariables|SetNew NewState)
  (return (Math|Boolean|ANDBoolean (.ReturnValue (Utilities|Map|Find (Variables|Default|GetAIStateProperty) (LocalVariables|GetNew))) _returnvalue (>= (.Value (Utilities|Map|Find (Variables|Default|GetAIStateProperty) (LocalVariables|GetNew))) _value))))

(fn TryAcquireToken
  (Utilities|FlowControl|Sequence
    (:then_0
      (bind _rezult (Class|BPIGameState|HasToken(Message) (Game|GetGameState) (Variables|Default|GetPawnRef)))
      (if _rezult
        (return true)))
    (:then_1
      (bind _rezult_2 (Class|BPIGameState|AddToken(Message) (Game|GetGameState) (Variables|Default|GetPawnRef)))
      (return _rezult_2))))

(fn ReleaseToken
  (Class|BPIGameState|RemoveToken(Message) (Game|GetGameState) (Variables|Default|GetPawnRef)))

(fn AIConsumeHit
  (params (Stamp :type Integer))
  (LocalVariables|SetStampCount Stamp)
  (Utilities|FlowControl|Sequence
    (:then_0
      (if (> (LocalVariables|GetStampCount) (Variables|Default|GetHandledStamp))
        (Variables|Default|SetHandledStamp (LocalVariables|GetStampCount))))
    (:then_1
      (CallFunction|SyncBlackboard)
      (return (== (Variables|Default|GetHitStamp) (Variables|Default|GetHandledStamp))))))

(fn AIGetAIState
  (return (Variables|Default|GetCurrentState)))

(fn AIGetCurrentTarget
  (return (.AsActor (Utilities|Casting|CastToActor (AI|Components|Blackboard|GetValueasObject (Variables|Default|GetBlackBoard) (Variables|KeyName|GetTargetKeyName))))))

(fn AIGetHitStamp
  (return (Variables|Default|GetHitStamp)))

(fn AIIsAlive
  (bind _dead (Class|BPIAttribute|IsDead(Message) (Variables|Default|GetAttributeRef)))
  (return (not _dead)))

(fn AITryEnterState
  (params (NewState :type E_AIState%20Enum :default "NewEnumerator0"))
  (LocalVariables|SetNew NewState)
  (Utilities|FlowControl|Sequence
    (:then_0
      (if (Utilities|Enum|Equal(Enum) (Variables|Default|GetCurrentState) "NewEnumerator8")
        (return false)))
    (:then_1
      (bind _rezult (CallFunction|CaninNewState (LocalVariables|GetNew)))
      (if _rezult
        (CallFunction|ApplyState (LocalVariables|GetNew))
        (return true)))
    (:then_2
      (return false))))