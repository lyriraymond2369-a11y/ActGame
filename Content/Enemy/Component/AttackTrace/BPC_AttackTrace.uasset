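; Enemy combat component that plays data-table attack and hit-reaction montages and handles melee hit detection and grab executions.
; While the attack window is open, Tick box-traces from the hitbox's opening location to its current one, hitting each actor once.
; Hostile hits pass damage, knockback and feedback to other components through interface messages.
; Grabbable targets instead trigger a random enabled execution, positioned instantly or by motion warping, with a timed loop on both characters.
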(event Custom|PlayMontageByID
  (params (ID :type Name))
  ;[0.15 0.15 0.15 0.5 36] 中间事件
  (bind _returnvalue (Utilities|GetDataTableRow (Variables|DataTable|GetAttacks) ID)
    (:then
      (Utilities|FlowControl|Sequence
        (:then_0
          (Variables|Default|SetCuurentAttack _returnvalue))
        (:then_1
          (Utilities|IsValid (.Montage (Utilities|Struct|BreakST_AttackData (Variables|Default|GetCuurentAttack)))
            (:Is%20Valid
              (bind _mesh (Class|BPICharacterBase|GetMeshComponent(Message) (Variables|Default|GetOwner)))
              (Animation|Montage|PlayMontage _mesh (.Montage (Utilities|Struct|BreakST_AttackData (Variables|Default|GetCuurentAttack))) 1.0 0.0 (.SectionStart (Utilities|Struct|BreakST_AttackData (Variables|Default|GetCuurentAttack)))
                (:OnCompleted
                  (Default|CallOnMontageFinished)
                  (Class|BPIGameState|RemoveToken(Message) (Game|GetGameState) (Variables|Default|GetOwner))
                  (Class|BPIAI|AIReturntoInitialState(Message) (Variables|Default|GetAIComponent)))))))))))

(event Custom|ApplyAttack
  (params (Actor :type Actor%20Object%20Reference) (HitLoc :type Vector))
  (bind _cuurentattack (Variables|Default|GetCuurentAttack))
  (bind (_id _montage _sectionstart _next _cancelstart _damagerate _poiseddamagerate _hitstop _launchenemy _canuseinair _playgravity _launchself) (Utilities|Struct|BreakST_AttackData _cuurentattack))
  ;[0.15 0.15 0.15 0.5 36] 中间事件
  (Variables|中间变量|SetMiddleActor Actor)
  (Variables|中间变量|SetMiddleVector3 HitLoc)
  (if (not (== (Variables|中间变量|GetMiddleActor) (Variables|Default|GetOwner)))
    (bind _rezult (Class|BPICharacterBase|IsHostile(Message) (Variables|Default|GetOwner) (Variables|中间变量|GetMiddleActor)))
    (if _rezult
      (Utilities|FlowControl|Sequence
        (:then_0
          (bind _attack (Class|BPIAttribute|GetAttack(Message) (Variables|Default|GetAttribute)))
          (bind _poiseattack (Class|BPIAttribute|GetPoiseAttack(Message) (Variables|Default|GetAttribute)))
          (bind _postureattack (Class|BPIAttribute|GetPostureAttack(Message) (Variables|Default|GetAttribute))))
        (:then_1
          (bind _attribute (Class|BPICharacterBase|GetAttributeComponent(Message) (Variables|中间变量|GetMiddleActor)))
          (bind (_hitoutcome _bperfectblock _bisbroken _bperfectdodge) (Class|BPIAttribute|ReceiveDamage(Message) _attribute (Variables|Default|GetCuurentAttack) _attack _poiseattack (Transformation|GetActorLocation (Variables|Default|GetOwner)) (Variables|中间变量|GetMiddleVector3) _postureattack))
          (Variables|中间变量|SetMiddleHitOutCome _hitoutcome)
          (Variables|Default|SetPerfect%20Block _bperfectblock)
          (Variables|Default|SetbBroken _bisbroken)
          (Variables|Default|SetPerfect%20Dodge _bperfectdodge))
        (:then_2
          (bind _motor (Class|BPICharacterBase|GetMotorComponent(Message) (Variables|中间变量|GetMiddleActor)))
          (Class|BPIMotor|ApplyKnockback(Message) _motor (CallFunction|GetLaunchVector _launchenemy) false)
          (Class|BPIMotor|ApplyKnockback(Message) (Variables|Default|GetMotor) (CallFunction|GetLaunchVector _launchself) false))
        (:then_3
          (Class|BPICombatFeedBack|PlayHitFeedback(Message) (Variables|Default|GetFeedback) (Variables|中间变量|GetMiddleHitOutCome) (Variables|中间变量|GetMiddleVector3) (Variables|Default|GetPerfect%20Block) (Variables|中间变量|GetMiddleActor) (.HitStop (Utilities|Struct|BreakST_AttackData (Variables|Default|GetCuurentAttack)))))))))

(event Custom|AttackCommon
  ;[0.15 0.15 0.15 0.5 36] 中间事件
  (CallFunction|PlayMontagebyID "Common1"))

(event Custom|MontageFinished
  ;[0.15 0.15 0.15 0.5 36] 中间事件
  (bind _aicomponent (Class|BPIEnemyBase|GetAIComponent(Message) (Variables|Default|GetOwner)))
  (Class|BPIAI|AISetState(Message) _aicomponent "NewEnumerator0"))

(event Custom|OpenAttackWindow
  ;[0.15 0.15 0.15 0.5 36] 更新
  (if (Variables|Default|GetbWindowOpen)
    (bind _hitbox (Class|BPICharacterBase|GetHitBoxComponent(Message) (Variables|Default|GetOwner)))
    (bind (_outhits _returnvalue) (Class|KismetSystemLibrary|BoxTraceMulti (Variables|Default|GetPrevTraceLoc) (Transformation|GetWorldLocation _hitbox) (Components|Box|GetScaledBoxExtent _hitbox) "0, 0, 0" "TraceTypeQuery4" false (Variables|Default|GetAlreadyHit) "None" true))
    (if _returnvalue
      (for _array_element _outhits
        (Variables|中间变量|SetMiddleVector3 (.ImpactPoint (Collision|BreakHitResult _array_element)))
        (Variables|中间变量|SetMiddleActor (.HitActor (Collision|BreakHitResult _array_element)))
        (if (not (or (== (Variables|Default|GetOwner) (Variables|中间变量|GetMiddleActor)) (Utilities|Array|ContainsItem (Variables|Default|GetAlreadyHit) (Variables|中间变量|GetMiddleActor))))
          (Utilities|Array|Add (Variables|Default|GetAlreadyHit) (Variables|中间变量|GetMiddleActor))
          (bind _actorcomponent (Class|BPIPlayer|GetCombatComponent(Message) (Variables|中间变量|GetMiddleActor)))
          (bind _rezult (Class|BPIExecution|CanbeGrabbed(Message) _actorcomponent))
          (if _rezult
            (Variables|Default|SetbWindowOpen false)
            (CallFunction|HandleGrabTransition (Variables|中间变量|GetMiddleActor))
            (else
              (CallFunction|ApplyAttack (Variables|中间变量|GetMiddleActor) (Variables|中间变量|GetMiddleVector3)))))))))

(event Custom|OnMontageEnd
  (params (Montage :type Anim%20Montage%20Object%20Reference) (bInterrupted :type Boolean))
  (if (and (not bInterrupted) (== Montage (.Montage (Utilities|Struct|BreakST_AttackData (Variables|Default|GetCuurentAttack)))))
    (CallFunction|MontageFinished)))

(event Custom|OnGrabLoopEnd
  (bind _currentgrabdata (Variables|投技|GetCurrentGrabData))
  (bind (_movetype _attackermontage _victimmontage _targetlocationoffset _bfacevictim _loopduration _randomweight _benabled _startsectionname _endsectionname) (Utilities|Struct|BreakST_GrabMoveData _currentgrabdata))
  ;[0.15 0.15 0.15 0.5 36] 接口事件
  (if (Variables|投技|GetbGrabActive)
    (if (Animation|Montage|MontageIsPlaying (Variables|Default|GetAnimInst) (.AttackerMontage (Utilities|Struct|BreakST_GrabMoveData (Variables|投技|GetCurrentGrabData))))
      (Ability|Animation|MontageJumptoSection (Variables|Default|GetAnimInst) _endsectionname _attackermontage)
      (bind _actorcomponent (Class|BPIPlayer|GetCombatComponent(Message) (Variables|投技|GetGrabVictim)))
      (Class|BPIExecution|JumpExecutiontoEnd(Message) _actorcomponent)
      (Utilities|Time|ClearandInvalidateTimerbyHandle (Variables|投技|GetGrabTimerHandle)))))

(event Custom|HandleGrabTransition
  (params (Victim :type Actor%20Object%20Reference))
  ;[0.15 0.15 0.15 0.5 36] 中间事件
  (Variables|中间变量|SetMiddleActor Victim)
  (if (not (Variables|投技|GetbGrabActive))
    (Utilities|IsValid (Variables|中间变量|GetMiddleActor)
      (:Is%20Valid
        (bind _name (CallFunction|GetRandomCurrentGrabRowName))
        (Variables|投技|SetCurrentGrabRowName _name)
        (Utilities|FlowControl|Sequence
          (:then_0
            (bind _returnvalue (Utilities|GetDataTableRow (Variables|数据表格|GetExecutions) (Variables|投技|GetCurrentGrabRowName))
              (:then
                (bind _output_get (Variables|投技|SetCurrentGrabData _returnvalue))
                (Variables|投技|SetGrabLoopDuration (.LoopDuration (Utilities|Struct|BreakST_GrabMoveData _output_get)))
                (Variables|投技|SetbGrabActive true)
                (Variables|投技|SetGrabVictim (Variables|中间变量|GetMiddleActor))
                (Variables|投技|SetbGrabLoopStarted false)
                (Utilities|Time|ClearandInvalidateTimerbyHandle (Variables|投技|GetGrabTimerHandle)))))
          (:then_1
            (switch Utilities|FlowControl|Switch|SwitchonE_GrabMoveType (.MoveType (Utilities|Struct|BreakST_GrabMoveData (Variables|投技|GetCurrentGrabData)))
              (:NewEnumerator0
                (Transformation|SetActorLocationAndRotation (Variables|Default|GetOwner) (.Location (CallFunction|GetGrabLocationandRotation (.TargetLocationOffset (Utilities|Struct|BreakST_GrabMoveData (Variables|投技|GetCurrentGrabData))) (Variables|投技|GetGrabVictim) (.bFaceVictim (Utilities|Struct|BreakST_GrabMoveData (Variables|投技|GetCurrentGrabData))))) (.Rotation (CallFunction|GetGrabLocationandRotation (.TargetLocationOffset (Utilities|Struct|BreakST_GrabMoveData (Variables|投技|GetCurrentGrabData))) (Variables|投技|GetGrabVictim) (.bFaceVictim (Utilities|Struct|BreakST_GrabMoveData (Variables|投技|GetCurrentGrabData)))))))
              (:NewEnumerator1
                (Class|MotionWarpingComponent|AddorUpdateWarpTargetfromLocationandRotation (Variables|Default|GetMotion%20Warping) "GrabWarp" (.Location (CallFunction|GetGrabLocationandRotation (.TargetLocationOffset (Utilities|Struct|BreakST_GrabMoveData (Variables|投技|GetCurrentGrabData))) (Variables|投技|GetGrabVictim) (.bFaceVictim (Utilities|Struct|BreakST_GrabMoveData (Variables|投技|GetCurrentGrabData))))) (.Rotation (CallFunction|GetGrabLocationandRotation (.TargetLocationOffset (Utilities|Struct|BreakST_GrabMoveData (Variables|投技|GetCurrentGrabData))) (Variables|投技|GetGrabVictim) (.bFaceVictim (Utilities|Struct|BreakST_GrabMoveData (Variables|投技|GetCurrentGrabData)))))))))
          (:then_2
            (Animation|Montage|PlayMontage (Variables|Default|GetMesh) (.AttackerMontage (Utilities|Struct|BreakST_GrabMoveData (Variables|投技|GetCurrentGrabData))) 1.0 0.0 (.StartSectionName (Utilities|Struct|BreakST_GrabMoveData (Variables|投技|GetCurrentGrabData)))
              (:OnCompleted
                (Class|BPIAI|AISetState(Message) (Variables|Default|GetAIComponent) "NewEnumerator0")
                (Variables|投技|SetbGrabActive false))))
          (:then_3
            (bind _actorcomponent (Class|BPIPlayer|GetCombatComponent(Message) (Variables|投技|GetGrabVictim)))
            (Class|BPIExecution|PlayExecutionVictim(Message) _actorcomponent (Variables|投技|GetCurrentGrabRowName))))))))

(event EventBeginPlay
  (bind _as角色 (Utilities|Casting|CastToCharacter (Components|GetOwner)))
  (bind _output_get (Variables|Default|SetOwner _as角色))
  (bind _mesh (Class|BPICharacterBase|GetMeshComponent(Message) _output_get))
  (bind _output_get_2 (Variables|Default|SetMesh _mesh))
  (bind _output_get_3 (Variables|Default|SetAnimInst (Components|SkeletalMesh|GetAnimInstance _output_get_2)))
  (EventDispatchers|BindEventtoOnMontageEnded _output_get_3 (delegate Custom|OnMontageEnd))
  (bind _feedback (Class|BPICharacterBase|GetCombatFeedbackComponent(Message) (Variables|Default|GetOwner)))
  (Variables|Default|SetFeedback _feedback)
  (bind _motor (Class|BPICharacterBase|GetMotorComponent(Message) (Variables|Default|GetOwner)))
  (Variables|Default|SetMotor _motor)
  (bind _aicomponent (Class|BPIEnemyBase|GetAIComponent(Message) (Variables|Default|GetOwner)))
  (Variables|Default|SetAIComponent _aicomponent)
  (bind _charactermovement (Class|BPICharacterBase|GetCharacterMovement(Message) (Variables|Default|GetOwner)))
  (Variables|Default|SetCharacter%20Movement _charactermovement)
  (bind _attribute (Class|BPICharacterBase|GetAttributeComponent(Message) (Variables|Default|GetOwner)))
  (Variables|Default|SetAttribute _attribute)
  (bind _motionwarping (Class|BPICharacterBase|GetMotionWarpingComponent(Message) (Variables|Default|GetOwner)))
  (Variables|Default|SetMotion%20Warping _motionwarping))

(event EventTick
  (params (DeltaSeconds :type Float%20%28single-precision%29))
  (CallFunction|OpenAttackWindow))

(event EventOnAttackWindow
  (params (On :type Boolean))
  ;[0.15 0.15 0.15 0.5 36] 接口事件
  (bind _output_get (Variables|Default|SetbWindowOpen On))
  (if _output_get
    (Utilities|Array|Clear (Variables|Default|GetAlreadyHit))
    (bind _hitbox (Class|BPICharacterBase|GetHitBoxComponent(Message) (Variables|Default|GetOwner)))
    (Variables|Default|SetPrevTraceLoc (Transformation|GetWorldLocation _hitbox))
    (Collision|SetCollisionEnabled _hitbox "NoCollision")
    (Audio|PlaySoundatLocation "/Game/ThirdParty/Sound/Sword/SwordWhoosh.SwordWhoosh" (Variables|Default|GetPrevTraceLoc) "0, 0, 0" 0.7 1.0 0.2 0 0 0 0)))

(event EventAttackbyType
  (params (AttackType :type E_AttackType%20Enum :default "NewEnumerator0"))
  ;[0.15 0.15 0.15 0.5 36] 接口事件
  (switch Utilities|FlowControl|Switch|SwitchonE_AttackType AttackType
    (:NewEnumerator0
      (CallFunction|AttackCommon))))

(event EventPlayHitMontage
  (params (State :type E_AIState%20Enum :default "NewEnumerator0") (Direction :type E_HitDirection%20Enum :default "NewEnumerator0"))
  ;[0.15 0.15 0.15 0.5 36] 接口事件
  (Variables|中间变量|SetMiddleAIState State)
  (Variables|中间变量|SetMiddleHitDirection Direction)
  (Utilities|IsValid (Variables|数据表格|GetHitDataTable)
    (:Is%20Valid
      (bind _returnvalue (Utilities|GetDataTableRow (Variables|数据表格|GetHitDataTable) (Utilities|String|StringToName (Utilities|String|Append (Utilities|String|MakeLiteralString (Utilities|Select :Index (Variables|中间变量|GetMiddleAIState) :NewEnumerator0 "" :NewEnumerator7 "" :NewEnumerator8 "" :NewEnumerator9 "" :NewEnumerator10 "HitLight" :NewEnumerator11 "HitHeavy" :NewEnumerator12 "")) "_" (Utilities|String|MakeLiteralString (Utilities|Select :Index (Variables|中间变量|GetMiddleHitDirection) :NewEnumerator0 "Front" :NewEnumerator1 "Back" :NewEnumerator2 "Left" :NewEnumerator3 "Right")))))
        (:then
          (bind _mesh (Class|BPICharacterBase|GetMeshComponent(Message) (Variables|Default|GetOwner)))
          (Animation|Montage|PlayMontage _mesh (.Montage (Utilities|Struct|BreakST_AttackData _returnvalue)) 1.0 0.0 (.SectionStart (Utilities|Struct|BreakST_AttackData _returnvalue))
            (:OnCompleted
              (Default|CallOnMontageFinished)
              (Class|BPIGameState|RemoveToken(Message) (Game|GetGameState) (Variables|Default|GetOwner))
              (Class|BPIAI|AIReturntoInitialState(Message) (Variables|Default|GetAIComponent)))))))))

(event EventOnGrabLoopStarted
  ;[0.15 0.15 0.15 0.5 36] 接口事件
  (if (Variables|投技|GetbGrabActive)
    (if (not (Variables|投技|GetbGrabLoopStarted))
      (Variables|投技|SetbGrabLoopStarted true)
      (Utilities|Time|ClearandInvalidateTimerbyHandle (Variables|投技|GetGrabTimerHandle))
      (bind _returnvalue (Utilities|Time|SetTimerbyEvent (delegate Custom|OnGrabLoopEnd) (.LoopDuration (Utilities|Struct|BreakST_GrabMoveData (Variables|投技|GetCurrentGrabData)))))
      (Variables|投技|SetGrabTimerHandle _returnvalue))))

(event EventOnGrabDamage
  ;[0.15 0.15 0.15 0.5 36] 接口事件
  (Class|BPICombatFeedBack|PlayGrabImpactSound(Message) (Variables|Default|GetFeedback)))

(fn GetLaunchVector
  (params (Vector3 :type Vector))
  (bind (_x _y _z) (Math|Vector|BreakVector Vector3))
  (bind _owner (Variables|Default|GetOwner))
  (return (+ (* (Transformation|GetActorForwardVector _owner) _x) (* (Transformation|GetActorRightVector _owner) _y) (* (Transformation|GetActorUpVector _owner) _z))))

(fn GetGrabLocationandRotation
  (params (Offset :type Vector) (Victim :type Actor%20Object%20Reference) (bFaceVictim :type Boolean))
  (LocalVariables|SetVictimOffset Offset)
  (LocalVariables|SetActor Victim)
  (LocalVariables|SetFace bFaceVictim)
  (LocalVariables|SetFinalLocation (+ (Transformation|GetActorLocation (LocalVariables|GetActor)) (* (Transformation|GetActorForwardVector (LocalVariables|GetActor)) (.X (Math|Vector|BreakVector (LocalVariables|GetVictimOffset)))) (* (Transformation|GetActorRightVector (LocalVariables|GetActor)) (.Y (Math|Vector|BreakVector (LocalVariables|GetVictimOffset)))) (* (Transformation|GetActorUpVector (LocalVariables|GetActor)) (.Z (Math|Vector|BreakVector (LocalVariables|GetVictimOffset))))))
  (return (LocalVariables|GetFinalLocation) (select (LocalVariables|GetFace) (Math|Rotator|FindLookatRotation (LocalVariables|GetFinalLocation) (Transformation|GetActorLocation (LocalVariables|GetActor))) (Transformation|GetActorRotation (Variables|Default|GetOwner)))))

(fn GetRandomCurrentGrabRowName
  (bind _outrownames (DataTable|GetDataTableRowNames (Variables|数据表格|GetExecutions)))
  (for _array_element _outrownames
    (bind _output_get (LocalVariables|SetCuurentName _array_element))
    (bind _returnvalue (Utilities|GetDataTableRow (Variables|数据表格|GetExecutions) _output_get)
      (:then
        (if (.bEnabled (Utilities|Struct|BreakST_GrabMoveData _returnvalue))
          (Utilities|Array|Add (LocalVariables|GetEnabledRowNames) (LocalVariables|GetCuurentName))))))
  (return (.OutItem (Utilities|Array|Random (LocalVariables|GetEnabledRowNames)))))