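; Training dummy enemy that gives brief visual feedback when hit, with no damage or health logic.
; The EnterHit interface event swaps the mesh to a hit material, nudges it horizontally toward the hit location and slightly enlarges the actor.
; After a very short delay it restores the common material, applies a reverse offset and resets the scale.
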(event EventBeginPlay)

(event Collision|EventActorBeginOverlap
  (params (OtherActor :type Actor%20Object%20Reference)))

(event EventTick
  (params (DeltaSeconds :type Float%20%28single-precision%29)))

(event EventEnterHit
  (params (HitType :type E_ActionState%20Enum :default "NewEnumerator0") (HitLoc :type Vector :default "0, 0, 0"))
  (bind _returnvalue (Transformation|GetActorLocation))
  (bind _returnvalue_2 (- HitLoc _returnvalue))
  (bind _returnvalue_3 (Math|Vector|Normalize _returnvalue_2))
  (bind _returnvalue_4 (* _returnvalue_3 5.0))
  (bind _returnvalue_5 (Math|Vector|MakeVector (.x _returnvalue_4) (.y _returnvalue_4) 0.0))
  ;[0.15 0.15 0.15 0.5 36] 接口事件
  (Utilities|FlowControl|Sequence
    (:then_0
      (Rendering|Material|SetMaterial (Variables|Default|GetStaticMesh) 0 (Variables|Default|GetHitMaterial))
      (Transformation|AddWorldOffset (Variables|Default|GetStaticMesh) _returnvalue_5 false false)
      (Transformation|SetActorScale3D "1.100000,1.100000,1.100000"))
    (:then_1
      (Utilities|FlowControl|Delay 0.05)
      (Rendering|Material|SetMaterial (Variables|Default|GetStaticMesh) 0 (Variables|Default|GetCommonMaterial))
      (Transformation|AddWorldOffset (Variables|Default|GetStaticMesh) (* _returnvalue_5 -1.0) false false)
      (Transformation|SetActorScale3D "1.000000,1.000000,1.000000"))))

(fn ConstructionScript
  (|CallParentFunction))