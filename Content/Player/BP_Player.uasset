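; Player character for melee combat, handling Enhanced Input movement, attacks, jump, dodge, guard and lock-on through components it exposes via getters.
; Action presses are pushed to an input buffer, which Tick consumes when the action state permits, then forwards to the combat component.
; BeginPlay spawns a sword, attaches it to the hand socket and takes its attribute bonus and hitbox.
; A looping timer spawns capped pose-copy afterimages.
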(event Custom|InitMovement
  ;[0.15 0.15 0.15 0.5 36] 初始化
  (Variables|/Script/Engine.CharacterMovementComponent|SetMaxWalkSpeed (Variables|Character|GetCharacterMovement) (Variables|速度|GetWalkSpeed))
  (Variables|状态|SetMoveState "NewEnumerator0"))

(event Custom|UpdateMoveState
  ;[0.15 0.15 0.15 0.5 36] 更新
  (if (<= (Class|KismetMathLibrary|VSize2DSquared (Variables|Default|GetAction%20Value)) 0.0)
    (Variables|状态|SetMoveState "NewEnumerator0")
    (else
      (Variables|状态|SetMoveState (select (Variables|状态|GetIsRun) "NewEnumerator2" "NewEnumerator1")))))

(event Custom|ClearNoUseGhost
  ;[0.15 0.15 0.15 0.5 36] 中间事件
  (for _array_element (Variables|残影|GetActiveGhosts)
    (Utilities|IsValid _array_element
      (:Is%20Not%20Valid
        (Utilities|Array|Add (Variables|残影|GetRemovedGhosts) _array_element))))
  (for _array_element_2 (Variables|残影|GetRemovedGhosts)
    (Utilities|Array|RemoveItem (Variables|残影|GetActiveGhosts) _array_element_2))
  (Utilities|Array|Clear (Variables|残影|GetRemovedGhosts)))

(event Custom|UpdateMoveSpeed
  ;[0.15 0.15 0.15 0.5 36] 更新
  (bind _actionstate (Class|BPIActionState|GetActionState(Message) (Variables|Default|GetBPC_ActionState)))
  (if (Utilities|Enum|NotEqual(Enum) _actionstate "NewEnumerator8")
    (bind _actionstate_2 (Class|BPIActionState|GetActionState(Message) (Variables|Default|GetBPC_ActionState)))
    (if (Utilities|Enum|Equal(Enum) _actionstate_2 "NewEnumerator0")
      (Variables|/Script/Engine.CharacterMovementComponent|SetMaxWalkSpeed (Variables|Character|GetCharacterMovement) (Utilities|Select :Index (Variables|状态|GetMoveState) :NewEnumerator0 1.6e+02 :NewEnumerator1 (Variables|速度|GetWalkSpeed) :NewEnumerator2 (Variables|速度|GetRunSpeed))))
    (else
      (Variables|/Script/Engine.CharacterMovementComponent|SetMaxWalkSpeed (Variables|Character|GetCharacterMovement) 2e+02))))

(event Custom|InitWeapon
  ;[0.15 0.15 0.15 0.5 36] 初始化
  (bind _returnvalue (Game|SpawnActorfromClass "/Game/Code/Weapon/BP_Player_Sword.BP_Player_Sword_C" (Math|Transform|MakeTransform "0, 0, 0" "0, 0, 0" "1.000000,1.000000,1.000000") "Undefined" "MultiplyWithRoot" 0 5.0 0))
  (bind _output_get (Variables|Default|SetWeapon _returnvalue))
  (Transformation|AttachComponentToComponent _output_get (Variables|Character|GetMesh) "Weapon_R" "KeepRelative" "KeepRelative" "KeepRelative" true)
  (CallFunction|FixedUpdateAttributeComponent)
  (bind _hitbox (Class|BPIWeaponBase|GetWeaponHitBox(Message) (Variables|Default|GetWeapon)))
  (Variables|Default|SetHit%20Box _hitbox))

(event Custom|FixedUpdateAttributeComponent
  (bind _weapon (Variables|Default|GetWeapon))
  ;[0.15 0.15 0.15 0.5 36] 更改时更新
  (bind _weaponbonus (Class|BPIWeaponBase|GetWeaponBonus(Message) _weapon))
  (Class|BPIAttribute|AddBonus(Message) (Variables|Default|GetBPC_Attribute) (select (Utilities|IsValid _weapon) _weaponbonus 0.0)))

(event Custom|UpdateLightState
  ;[0.15 0.15 0.15 0.5 36] 更新
  (bind _actionstate (Class|BPIActionState|GetActionState(Message) (Variables|Default|GetBPC_ActionState)))
  (switch Utilities|FlowControl|Switch|SwitchonE_ActionState _actionstate
    (:NewEnumerator0
      _)
    (:NewEnumerator1
      _)
    (:NewEnumerator2
      _)
    (:NewEnumerator3
      _))
  (bind _rezult (Class|BPIBufferInput|Comsume(Message) (Variables|Default|GetBPC_BufferInput) "NewEnumerator0"))
  (if _rezult
    (Class|BPICombat|DoLight(Message) (Variables|Default|GetBPC_Combat))))

(event Custom|UpdateDodgeState
  ;[0.15 0.15 0.15 0.5 36] 更新
  (bind _actionstate (Class|BPIActionState|GetActionState(Message) (Variables|Default|GetBPC_ActionState)))
  (switch Utilities|FlowControl|Switch|SwitchonE_ActionState _actionstate
    (:NewEnumerator0
      _)
    (:NewEnumerator1
      _)
    (:NewEnumerator2
      _)
    (:NewEnumerator4
      _)
    (:NewEnumerator8
      _))
  (bind _rezult (Class|BPIBufferInput|Comsume(Message) (Variables|Default|GetBPC_BufferInput) "NewEnumerator2"))
  (if _rezult
    (bind _direction (CallFunction|GetDodgeDirection))
    (Class|BPICombat|DoDodge(Message) (Variables|Default|GetBPC_Combat) _direction)))

(event Custom|UpdateJumpState
  ;[0.15 0.15 0.15 0.5 36] 更新
  (bind _actionstate (Class|BPIActionState|GetActionState(Message) (Variables|Default|GetBPC_ActionState)))
  (switch Utilities|FlowControl|Switch|SwitchonE_ActionState _actionstate
    (:NewEnumerator0
      _)
    (:NewEnumerator2
      _)
    (:NewEnumerator3
      _))
  (bind _rezult (Class|BPIBufferInput|Comsume(Message) (Variables|Default|GetBPC_BufferInput) "NewEnumerator3"))
  (if _rezult
    (Class|BPICombat|DoJump(Message) (Variables|Default|GetBPC_Combat))))

(event Custom|UpdateHeavyState
  ;[0.15 0.15 0.15 0.5 36] 更新
  (bind _actionstate (Class|BPIActionState|GetActionState(Message) (Variables|Default|GetBPC_ActionState)))
  (switch Utilities|FlowControl|Switch|SwitchonE_ActionState _actionstate
    (:NewEnumerator0
      _)
    (:NewEnumerator1
      _)
    (:NewEnumerator2
      _)
    (:NewEnumerator3
      _))
  (bind _rezult (Class|BPIBufferInput|Comsume(Message) (Variables|Default|GetBPC_BufferInput) "NewEnumerator1"))
  (if _rezult
    (Class|BPICombat|DoHeavy(Message) (Variables|Default|GetBPC_Combat))))

(event Custom|SpawnGhost
  ;[0.15 0.15 0.15 0.5 36] 接口事件
  (CallFunction|ClearNoUseGhost)
  (if (< (Utilities|Array|Length (Variables|残影|GetActiveGhosts)) (Variables|残影|GetMaxGhosts))
    (bind _returnvalue (Game|SpawnActorfromClass (Variables|残影|GetAfterimageClass) (Transformation|GetWorldTransform (Variables|Character|GetMesh)) "AlwaysSpawn" "MultiplyWithRoot" 0 0))
    (Class|BPIAfterimage|CopyPosefrom(Message) _returnvalue (Variables|Character|GetMesh))
    (Utilities|Array|Add (Variables|残影|GetActiveGhosts) _returnvalue)))

(event Input|EnhancedActionEvents|EnhancedInputActionIA_Move
  (params (ActionValue :type Vector%202D%20Structure) (ElapsedSeconds :type Float%20%28double-precision%29) (TriggeredSeconds :type Float%20%28double-precision%29) (InputAction :type Input%20Action%20Object%20Reference :default "/Game/Player/Input/IA_Move.IA_Move"))
  (bind _camera (Variables|Default|GetCamera))
  (bind _camera_2 (Variables|Default|GetCamera))
  (bind _returnvalue (Math|Vector|GetForwardVector _camera))
  (bind _returnvalue_2 (Math|Vector|GetRightVector _camera_2))
  ;[0.15 0.15 0.15 0.5 36] 输入
  ;;[0.15 0.15 0.15 0.5] 角色移动
  (:Triggered
    (bind _output_get (Variables|Default|SetAction%20Value ActionValue))
    (bind _actionstate (Class|BPIActionState|GetActionState(Message) (Variables|Default|GetBPC_ActionState)))
    (if (Utilities|Array|ContainsItem (Utilities|Array|MakeArray "NewEnumerator0" "NewEnumerator8") _actionstate)
      (Pawn|Input|AddMovementInput (Math|Vector|MakeVector (.x _returnvalue) (.y _returnvalue) 0.0) (.X (Math|Vector2D|BreakVector2D _output_get)) false)
      (Pawn|Input|AddMovementInput (Math|Vector|MakeVector (.x _returnvalue_2) (.y _returnvalue_2) 0.0) (.Y (Math|Vector2D|BreakVector2D _output_get)) false)))
  (:Completed
    (Variables|Default|SetAction%20Value "")))

(event Input|EnhancedActionEvents|EnhancedInputActionIA_Look
  (params (ActionValue :type Vector%202D%20Structure) (ElapsedSeconds :type Float%20%28double-precision%29) (TriggeredSeconds :type Float%20%28double-precision%29) (InputAction :type Input%20Action%20Object%20Reference :default "/Game/Player/Input/IA_Look.IA_Look"))
  (bind (_x _y) (Math|Vector2D|BreakVector2D ActionValue))
  ;[0.15 0.15 0.15 0.5 36] 输入
  ;;[0.15 0.15 0.15 0.5] 角色视角移动
  (Pawn|Input|AddControllerYawInput (* (Variables|Default|GetMouseSensitive) _x))
  (Pawn|Input|AddControllerPitchInput (* _y (Variables|Default|GetMouseSensitive))))

(event Input|EnhancedActionEvents|EnhancedInputActionIA_Run
  (params (ActionValue :type Boolean) (ElapsedSeconds :type Float%20%28double-precision%29) (TriggeredSeconds :type Float%20%28double-precision%29) (InputAction :type Input%20Action%20Object%20Reference :default "/Game/Player/Input/IA_Run.IA_Run"))
  ;[0.15 0.15 0.15 0.5 36] 输入
  ;;[0.15 0.15 0.15 0.5] 奔跑
  (:Started
    (Variables|状态|SetIsRun true))
  (:Completed
    (Variables|状态|SetIsRun false)))

(event Input|EnhancedActionEvents|EnhancedInputActionIA_Jump
  (params (ActionValue :type Boolean) (ElapsedSeconds :type Float%20%28double-precision%29) (TriggeredSeconds :type Float%20%28double-precision%29) (InputAction :type Input%20Action%20Object%20Reference :default "/Game/Player/Input/IA_Jump.IA_Jump"))
  ;[0.15 0.15 0.15 0.5 36] 输入
  (:Started
    (Class|BPIBufferInput|Push(Message) (Variables|Default|GetBPC_BufferInput) "NewEnumerator3"))
  (:Completed
    (Character|StopJumping)))

(event Input|EnhancedActionEvents|EnhancedInputActionIA_Light
  (params (ActionValue :type Boolean) (ElapsedSeconds :type Float%20%28double-precision%29) (TriggeredSeconds :type Float%20%28double-precision%29) (InputAction :type Input%20Action%20Object%20Reference :default "/Game/Player/Input/IA_Light.IA_Light"))
  ;[0.15 0.15 0.15 0.5 36] 输入
  (:Started
    (Class|BPIBufferInput|Push(Message) (Variables|Default|GetBPC_BufferInput) "NewEnumerator0")))

(event Input|EnhancedActionEvents|EnhancedInputActionIA_Heavy
  (params (ActionValue :type Boolean) (ElapsedSeconds :type Float%20%28double-precision%29) (TriggeredSeconds :type Float%20%28double-precision%29) (InputAction :type Input%20Action%20Object%20Reference :default "/Game/Player/Input/IA_Heavy.IA_Heavy"))
  ;[0.15 0.15 0.15 0.5 36] 输入
  (:Started
    (Class|BPIBufferInput|Push(Message) (Variables|Default|GetBPC_BufferInput) "NewEnumerator1")))

(event Input|EnhancedActionEvents|EnhancedInputActionIA_Dodge
  (params (ActionValue :type Boolean) (ElapsedSeconds :type Float%20%28double-precision%29) (TriggeredSeconds :type Float%20%28double-precision%29) (InputAction :type Input%20Action%20Object%20Reference :default "/Game/Player/Input/IA_Dodge.IA_Dodge"))
  ;[0.15 0.15 0.15 0.5 36] 输入
  (:Started
    (Class|BPIBufferInput|Push(Message) (Variables|Default|GetBPC_BufferInput) "NewEnumerator2")))

(event Input|EnhancedActionEvents|EnhancedInputActionIA_Aim
  (params (ActionValue :type Boolean) (ElapsedSeconds :type Float%20%28double-precision%29) (TriggeredSeconds :type Float%20%28double-precision%29) (InputAction :type Input%20Action%20Object%20Reference :default "/Game/Player/Input/IA_Aim.IA_Aim"))
  ;[0.15 0.15 0.15 0.5 36] 输入
  (:Started
    (bind _rezult (CallFunction|IsBlock))
    (if (not _rezult)
      (Class|BPILockon|HardLockPress(Message) (Variables|Default|GetBPC_LockOn))
      (CallFunction|IntoHardLockState)))
  (:Completed
    (bind _rezult_2 (CallFunction|IsBlock))
    (if (not _rezult_2)
      (Class|BPILockon|HardLockRelease(Message) (Variables|Default|GetBPC_LockOn))
      (CallFunction|OutHardLockState))))

(event Input|EnhancedActionEvents|EnhancedInputActionIA_Block
  (params (ActionValue :type Boolean) (ElapsedSeconds :type Float%20%28double-precision%29) (TriggeredSeconds :type Float%20%28double-precision%29) (InputAction :type Input%20Action%20Object%20Reference :default "/Game/Player/Input/IA_Block.IA_Block"))
  ;[0.15 0.15 0.15 0.5 36] 输入
  (:Started
    (bind _rezult (Class|BPIActionState|TryEnterState(Message) (Variables|Default|GetBPC_ActionState) "NewEnumerator8"))
    (if _rezult
      (Class|BPIAttribute|EnterGuard(Message) (Variables|Default|GetBPC_Attribute))
      (Class|BPILockon|HardLockPress(Message) (Variables|Default|GetBPC_LockOn))
      (bind _lockstate (Class|BPILockon|GetLockState(Message) (Variables|Default|GetBPC_LockOn)))
      (if (Utilities|Enum|Equal(Enum) _lockstate "NewEnumerator2")
        (CallFunction|IntoHardLockState))))
  (:Completed
    (CallFunction|OutBlock)))

(event EventBeginPlay
  (bind _asbp_player_controller (Utilities|Casting|CastToBP_PlayerController (Pawn|GetController)))
  (Input|AddMappingContext (PlayerController|LocalPlayerSubsystems|GetEnhancedInputLocalPlayerSubsystem _asbp_player_controller) "/Game/Player/Input/IMC_Player.IMC_Player" 0 "(bIgnoreAllPressedKeysUntilRelease=True,bForceImmediately=False,bNotifyUserSettings=False)")
  (CallFunction|InitMovement)
  (CallFunction|InitWeapon))

(event EventApplyImpulse
  (params (Vector :type Vector :default "0, 0, 0") (XYOverride :type Boolean) (ZOverride :type Boolean))
  ;[0.15 0.15 0.15 0.5 36] 接口事件
  (Character|LaunchCharacter Vector XYOverride ZOverride))

(event EventTick
  (params (DeltaSeconds :type Float%20%28single-precision%29))
  (Variables|Default|SetDelta%20Seconds DeltaSeconds)
  (CallFunction|UpdateMoveState)
  (CallFunction|UpdateMoveSpeed)
  (CallFunction|UpdateLightState)
  (CallFunction|UpdateHeavyState)
  (CallFunction|UpdateJumpState)
  (CallFunction|UpdateDodgeState)
  (bind _actionstate (Class|BPIActionState|GetActionState(Message) (Variables|Default|GetBPC_ActionState)))
  (Development|PrintString (Utilities|String|EnumtoString _actionstate) true true "(R=0.000000,G=0.660000,B=1.000000,A=1.000000)" 0.0))

(event EventOutBlock
  ;[0.15 0.15 0.15 0.5 36] 接口事件
  (bind _rezult (CallFunction|IsBlock))
  (if _rezult
    (Class|BPIActionState|SetState(Message) (Variables|Default|GetBPC_ActionState) "NewEnumerator0")
    (Class|BPILockon|HardLockRelease(Message) (Variables|Default|GetBPC_LockOn))
    (CallFunction|OutHardLockState)
    (Class|BPIAttribute|ExitGuard(Message) (Variables|Default|GetBPC_Attribute))
    (Class|BPICombat|SetLastGuardEndTime(Message) (Variables|Default|GetBPC_Combat) (Utilities|Time|GetGameTimeinSeconds))))

(event EventIntoHardLockState
  ;[0.15 0.15 0.15 0.5 36] 接口事件
  (Variables|/Script/Engine.CharacterMovementComponent|SetbOrientRotationToMovement (Variables|Character|GetCharacterMovement) false))

(event EventOutHardLockState
  ;[0.15 0.15 0.15 0.5 36] 接口事件
  (Variables|/Script/Engine.CharacterMovementComponent|SetbOrientRotationToMovement (Variables|Character|GetCharacterMovement) true))

(event EventStartJump
  ;[0.15 0.15 0.15 0.5 36] 接口事件
  (Character|Jump))

(event EventSetLockPlevisZ
  (params (Val :type Boolean))
  ;[0.15 0.15 0.15 0.5 36] 接口事件
  (Variables|Default|SetbLockPelvisZ Val))

(event EventStartAfterimage
  ;[0.15 0.15 0.15 0.5 36] 接口事件
  (Utilities|Time|ClearandInvalidateTimerbyHandle (Variables|残影|GetGhostTimerHandle))
  (Utilities|FlowControl|Sequence
    (:then_0
      (CallFunction|ClearNoUseGhost))
    (:then_1
      (bind _returnvalue (Utilities|Time|SetTimerbyEvent (delegate Custom|SpawnGhost) (Variables|残影|GetGhostInterval) true))
      (Variables|残影|SetGhostTimerHandle _returnvalue))))

(event EventStopAfterimage
  ;[0.15 0.15 0.15 0.5 36] 接口事件
  (Utilities|Time|ClearandInvalidateTimerbyHandle (Variables|残影|GetGhostTimerHandle)))

(event Input|KeyboardEvents|T
  (params (Key :type Key%20Structure :default "None")))

(fn ConstructionScript)

(fn IsBlock
  (bind _actionstate (Class|BPIActionState|GetActionState(Message) (Variables|Default|GetBPC_ActionState)))
  (return (Utilities|Enum|Equal(Enum) _actionstate "NewEnumerator8")))

(fn GetDodgeDirection
  (bind _action_value (Variables|Default|GetAction%20Value))
  (bind (_x _y) (Math|Vector2D|BreakVector2D _action_value))
  (Utilities|FlowControl|Sequence
    (:then_0
      (LocalVariables|SetInputX _x)
      (LocalVariables|SetInputY _y))
    (:then_1
      (if (== (LocalVariables|GetInputX) 1.0)
        (return "Front")
        (elif (== (LocalVariables|GetInputX) -1.0)
          (return "Back"))))
    (:then_2
      (if (== (LocalVariables|GetInputY) 1.0)
        (return "Right")
        (elif (== (LocalVariables|GetInputY) -1.0)
          (return "Left"))))
    (:then_3
      (bind _actor (Class|BPILockon|GetFocusTarget(Message) (Variables|Default|GetBPC_LockOn)))
      (return (select (Utilities|IsValid _actor) (Variables|Default|GetDefaultDodgeDirection) "Front")))))

(fn GetNormalwithOutZ
  (params (Val :type Vector))
  (bind (_x _y) (Math|Vector|BreakVector Val))
  (return (Math|Vector|Normalize (Math|Vector|MakeVector _x _y 0.0))))

(fn GetActionStateComponent
  (return (Variables|Default|GetBPC_ActionState)))

(fn GetAttributeComponent
  (return (Variables|Default|GetBPC_Attribute)))

(fn GetBufferInputComponent
  (return (Variables|Default|GetBPC_BufferInput)))

(fn GetCameraComponent
  (return (Variables|Default|GetCamera)))

(fn GetCameraDirectorComponent
  (return (Variables|Default|GetBPC_CameraDirector)))

(fn GetCharacterMovement
  (return (Variables|Character|GetCharacterMovement)))

(fn GetCombatComponent
  (return (Variables|Default|GetBPC_Combat)))

(fn GetCombatFeedbackComponent
  (return (Variables|Default|GetBPC_CombatFeedBack)))

(fn GetHitBoxComponent
  (return (Variables|Default|GetHit%20Box)))

(fn GetLockComponent
  (return (Variables|Default|GetBPC_LockOn)))

(fn GetMeshComponent
  (return (Variables|Character|GetMesh)))

(fn GetMotorComponent
  (return (Variables|Default|GetBPC_Motor)))

(fn GetWeapon
  (return (Variables|Default|GetWeapon)))

(fn IsCharacterDead
  (bind _dead (Class|BPIAttribute|IsDead(Message) (Variables|Default|GetBPC_Attribute)))
  (return _dead))

(fn IsHostile
  (params (Other :type Actor%20Object%20Reference))
  (bind _attribute (Class|BPICharacterBase|GetAttributeComponent(Message) Other))
  (bind _team (Class|BPIAttribute|GetTeam(Message) _attribute))
  (bind _team_2 (Class|BPIAttribute|GetTeam(Message) (Variables|Default|GetBPC_Attribute)))
  (return (Utilities|Enum|NotEqual(Enum) _team_2 _team)))