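; Player component that buffers typed inputs so they can be consumed within a time window.
; Push stores each input with game time plus Windows in parallel Keys and TImes arrays, dropping the oldest beyond ten.
; Consume removes the first match whose current-minus-stored time is within Windows, effectively twice Windows after the push.
; Peek reports whether the first match's stored time has already passed, without removing it.
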(event Custom|AddArrayItem
  (params (Input :type E_InputType%20Enum :default "NewEnumerator0") (time :type Float%20%28double-precision%29))
  ;[0.15 0.15 0.15 0.5 36] 中间事件
  (Utilities|Array|Add (Variables|Default|GetKeys) Input)
  (Utilities|Array|Add (Variables|Default|GetTImes) time))

(event Custom|RemoveArrayItem
  (params (Index :type Integer))
  ;[0.15 0.15 0.15 0.5 36] 中间事件
  (Utilities|Array|RemoveIndex (Variables|Default|GetKeys) Index)
  (Utilities|Array|RemoveIndex (Variables|Default|GetTImes) Index))

(event EventBeginPlay)

(event EventTick
  (params (DeltaSeconds :type Float%20%28single-precision%29)))

(event EventPush
  (params (Type :type E_InputType%20Enum :default "NewEnumerator0"))
  ;[0.15 0.15 0.15 0.5 36] 接口事件
  (CallFunction|AddArrayItem Type (+ (Utilities|Time|GetGameTimeinSeconds) (Variables|Default|GetWindows)))
  (if (> (Utilities|Array|Length (Variables|Default|GetKeys)) 10)
    (CallFunction|RemoveArrayItem)))

(fn Comsume
  (params (Type :type E_InputType%20Enum :default "NewEnumerator0"))
  (if (== (Utilities|Array|FindItem (Variables|Default|GetKeys) Type) -1)
    _
    (else
      (for (_array_element _array_index) (Variables|Default|GetKeys)
        (if (Utilities|Enum|Equal(Enum) _array_element Type)
          (LocalVariables|SetIndex _array_index)
          (if (<= (- (Utilities|Time|GetGameTimeinSeconds) (Utilities|Array|Get(acopy) (Variables|Default|GetTImes) (LocalVariables|GetIndex))) (Variables|Default|GetWindows))
            (CallFunction|RemoveArrayItem (LocalVariables|GetIndex))
            (return true))))))
  (return false))

(fn Peek
  (params (Input :type E_InputType%20Enum :default "NewEnumerator0"))
  (bind _keys (Variables|Default|GetKeys))
  (bind _returnvalue (Utilities|Array|FindItem _keys Input))
  (if (!= _returnvalue -1)
    (return (>= (Utilities|Time|GetGameTimeinSeconds) (Utilities|Array|Get(acopy) (Variables|Default|GetTImes) _returnvalue)))))