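; Player camera director component that plays combat camera shakes and a zoom-in close-up for perfect blocks.
; Shake requests pick a shake class by type (hit, block, perfect block, break, kill, perfect dodge), scaled by player distance between inner and outer radii and throttled by time.
; The close-up runs a Tick-driven In, Hold, Out phase machine that lerps camera FOV down from its base and back.
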(event Custom|UpdateCloseUpFOV
  ;[0.15 0.15 0.15 0.5 36] 更新
  (if (Variables|视野|GetbCloseUpActive)
    (switch Utilities|FlowControl|Switch|SwitchonE_CloseUpPhase (Variables|视野|GetCloseUpPhase)
      (:NewEnumerator0
        (CallFunction|CloseUpin))
      (:NewEnumerator1
        (CallFunction|CloseUpHold))
      (:NewEnumerator2
        (CallFunction|CloseUpOut)))))

(event Custom|CloseUp_In
  (bind _rezult (CallFunction|GetElapsed))
  (bind _closeupintime (Variables|视野|GetCloseUpInTime))
  (bind _returnvalue (/ _rezult _closeupintime))
  (bind _returnvalue_2 (Math|Float|Clamp(Float) _returnvalue))
  ;[0.15 0.15 0.15 0.5 36] 中间事件
  (Utilities|FlowControl|Sequence
    (:then_0
      (Camera|SetFieldOfView (Variables|Default|GetCamera) (Math|Float|Lerp (Variables|FOV|GetBaseFOV) (Variables|视野|GetTargetFOV) _returnvalue_2)))
    (:then_1
      (if (>= _returnvalue_2 1.0)
        (Variables|视野|SetCloseUpPhase "NewEnumerator1")
        (Variables|视野|SetCloseUpPhaseStartTime (Utilities|Time|GetGameTimeinSeconds))))))

(event Custom|CloseUp_Hold
  ;[0.15 0.15 0.15 0.5 36] 中间事件
  (Camera|SetFieldOfView (Variables|Default|GetCamera) (Variables|视野|GetTargetFOV))
  (if (>= (CallFunction|GetElapsed) (Variables|视野|GetCloseUpHoldTime))
    (Variables|视野|SetCloseUpPhase "NewEnumerator2")
    (Variables|视野|SetCloseUpPhaseStartTime (Utilities|Time|GetGameTimeinSeconds))))

(event Custom|CloseUp_Out
  (bind _rezult (CallFunction|GetElapsed))
  (bind _closeupouttime (Variables|视野|GetCloseUpOutTime))
  (bind _returnvalue (/ _rezult _closeupouttime))
  (bind _returnvalue_2 (Math|Float|Clamp(Float) _returnvalue))
  ;[0.15 0.15 0.15 0.5 36] 中间事件
  (Utilities|FlowControl|Sequence
    (:then_0
      (Camera|SetFieldOfView (Variables|Default|GetCamera) (Math|Float|Lerp (Variables|视野|GetTargetFOV) (Variables|FOV|GetBaseFOV) _returnvalue_2)))
    (:then_1
      (if (>= _returnvalue_2 1.0)
        (Camera|SetFieldOfView (Variables|Default|GetCamera) (Variables|FOV|GetBaseFOV))
        (Variables|视野|SetbCloseUpActive false)
        (Variables|视野|SetCloseUpPhase "NewEnumerator3")))))

(event EventBeginPlay
  (bind _output_get (Variables|Default|SetPlayerPawn (Game|Player|GetPlayerPawn 0)))
  (bind _camera (Class|BPIPlayer|GetCameraComponent(Message) _output_get))
  (bind _output_get_2 (Variables|Default|SetCamera _camera))
  (Variables|FOV|SetBaseFOV (Variables|/Script/Engine.CameraComponent|GetFieldOfView _output_get_2)))

(event EventTick
  (params (DeltaSeconds :type Float%20%28single-precision%29))
  (CallFunction|UpdateCloseUpFOV))

(event EventShake
  (params (Type :type E_CameraShakeType%20Enum :default "NewEnumerator0") (Location :type Vector :default "0, 0, 0") (Scale :type Float%20%28double-precision%29))
  ;[0.15 0.15 0.15 0.5 36] 接口事件
  (Variables|中间变量|SetMiddleEnum Type)
  (Variables|中间变量|SetMiddleVector3 Location)
  (Variables|中间变量|SetMiddleFloat Scale)
  (if (> (Variables|Default|GetShakeMultiplier) 0.0)
    (Utilities|IsValid (Variables|Default|GetPlayerPawn)
      (:Is%20Valid
        (bind _output_get (Variables|中间变量|SetMiddleFloat (* (|(1-((a-b)/(c-d))) (Math|Float|Clamp(Float) (Math|Vector|Distance(Vector) (Transformation|GetActorLocation (Variables|Default|GetPlayerPawn)) (Variables|中间变量|GetMiddleVector3)) (Variables|Default|GetShakeInnerRadius) (Variables|Default|GetShakeOuterRadius)) (Variables|Default|GetShakeInnerRadius) (Variables|Default|GetShakeOuterRadius) (Variables|Default|GetShakeInnerRadius)) (Variables|中间变量|GetMiddleFloat))))
        (if (> _output_get 0.01)
          (if (>= (- (Utilities|Time|GetGameTimeinSeconds) (Variables|Default|GetLastShakeEndTime)) (Variables|Default|GetMinShakeInterval))
            (Variables|Default|SetLastShakeEndTime (+ (Utilities|Time|GetGameTimeinSeconds) (Variables|Default|GetMinShakeInterval)))
            (CameraShakes|StartCameraShake (Game|GetPlayerCameraManager 0) (Utilities|Select :Index (Variables|中间变量|GetMiddleEnum) :NewEnumerator0 (Variables|Shake|GetShake_Hit) :NewEnumerator1 (Variables|Shake|GetShake_Block) :NewEnumerator2 (Variables|Shake|GetShake_PerfectBlock) :NewEnumerator3 (Variables|Shake|GetShake_Break) :NewEnumerator4 (Variables|Shake|GetShake_Kill) :NewEnumerator5 (Variables|Shake|GetShake_PerfectDodge)) (Variables|中间变量|GetMiddleFloat) "World" "0, 0, 0")))))))

(event EventPlayPerfectBlockCloseUp
  ;[0.15 0.15 0.15 0.5 36] 接口事件
  (if (not (Variables|视野|GetbCloseUpActive))
    (Variables|视野|SetbCloseUpActive true)
    (Variables|视野|SetCloseUpPhase "NewEnumerator0")
    (Variables|视野|SetCloseUpPhaseStartTime (Utilities|Time|GetGameTimeinSeconds))
    (Variables|视野|SetTargetFOV (- (Variables|FOV|GetBaseFOV) (Variables|FOV|GetCloseUpFOVDelta)))))

(fn GetElapsed
  (return (- (Utilities|Time|GetGameTimeinSeconds) (Variables|视野|GetCloseUpPhaseStartTime))))