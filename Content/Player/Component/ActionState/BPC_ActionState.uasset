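; Player component that holds the current action state, such as locomotion, jump, attack, dodge, guard, hit or dead, and arbitrates changes between them.
; TryEnterState applies per-state rules: allow lists, attack chaining in a cancel window, and priority comparison from ControlledStateProperty.
; ForceEnterState skips those rules but requires the cancel window and an uncontrolled current state.
; Tick returns Jump to Locomotion on landing, and timestamps drive dodge and guard cooldown checks.
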(event Custom|UpdateJumpState
  ;[0.15 0.15 0.15 0.5 36] 中间事件
  (if (and (Utilities|Enum|Equal(Enum) (Variables|Default|GetCurrentState) "NewEnumerator1") (not (AI|Components|NavMovement|IsFalling (Variables|Default|GetCharacter%20Movement))))
    (CallFunction|SetState "NewEnumerator0")))

(event EventBeginPlay
  (bind _output_get (Variables|Default|SetOwner (Components|GetOwner)))
  (bind _motor (Class|BPICharacterBase|GetMotorComponent(Message) _output_get))
  (Variables|Default|SetMotor _motor)
  (bind _attribute (Class|BPICharacterBase|GetAttributeComponent(Message) (Variables|Default|GetOwner)))
  (Variables|Default|SetAttribute _attribute)
  (bind _charactermovement (Class|BPICharacterBase|GetCharacterMovement(Message) (Variables|Default|GetOwner)))
  (Variables|Default|SetCharacter%20Movement _charactermovement)
  (bind _actorcomponent (Class|BPIPlayer|GetCombatComponent(Message) (Variables|Default|GetOwner)))
  (Variables|Default|SetCombat _actorcomponent))

(event EventTick
  (params (DeltaSeconds :type Float%20%28single-precision%29))
  (CallFunction|UpdateJumpState))

(event EventSetState
  (params (New :type E_ActionState%20Enum :default "NewEnumerator0"))
  ;[0.15 0.15 0.15 0.5 36] 接口事件
  (Variables|Default|SetCurrentState New)
  (Variables|Default|SetbCanCancel false))

(event EventSetCancelWindow
  (params (On :type Boolean))
  ;[0.15 0.15 0.15 0.5 36] 接口事件
  (Variables|Default|SetbCanCancel On))

(event EventUpdateDodgeCD
  (params (Time :type Float%20%28double-precision%29))
  ;[0.15 0.15 0.15 0.5 36] 接口事件
  (Variables|闪避|SetLastDodgeTime Time))

(event EventClearDodgeCD
  ;[0.15 0.15 0.15 0.5 36] 接口事件
  (Variables|闪避|SetLastDodgeTime -999.0))

(event EventUpdateGuardCD
  (params (Time :type Float%20%28double-precision%29))
  ;[0.15 0.15 0.15 0.5 36] 接口事件
  (Variables|格挡|SetLastGuardEndTime Time))

(event EventClearGuardCD
  ;[0.15 0.15 0.15 0.5 36] 接口事件
  (Variables|格挡|SetLastGuardEndTime -9999.0))

(fn CanTransitionto
  (params (NewState :type E_ActionState%20Enum :default "NewEnumerator0"))
  (LocalVariables|SetNew NewState)
  (switch Utilities|FlowControl|Switch|SwitchonE_ActionState (Variables|Default|GetCurrentState)
    (:NewEnumerator0
      (return true))
    (:NewEnumerator1
      (bind _rezult (转换条件|CaninNewStatefromJump (LocalVariables|GetNew)))
      (return _rezult))
    (:NewEnumerator2
      (bind _rezult_2 (转换条件|CaninNewStatefromAttack (LocalVariables|GetNew)))
      (if _rezult_2
        (return true)
        (elif (and (Variables|Default|GetbCanCancel) (Utilities|Enum|Equal(Enum) (LocalVariables|GetNew) "NewEnumerator2"))
          (return true)
          (else
            (return false)))))
    (:NewEnumerator3
      _)
    (:NewEnumerator4
      _)
    (:NewEnumerator5
      _)
    (:NewEnumerator6
      _)
    (:NewEnumerator7
      _)
    (:NewEnumerator8
      (return (Utilities|Map|Contains (Variables|Default|GetControlledStateProperty) (LocalVariables|GetNew)))))
  (bind _rezult_3 (CallFunction|TransStatebyProperty (LocalVariables|GetNew)))
  (return _rezult_3))

(fn CaninNewStatefromJump
  (params (new :type E_ActionState%20Enum :default "NewEnumerator0"))
  (return (Utilities|Array|ContainsItem (Utilities|Array|MakeArray "NewEnumerator0" "NewEnumerator2" "NewEnumerator3" "NewEnumerator4" "NewEnumerator5" "NewEnumerator6" "NewEnumerator7") new)))

(fn CaninNewStatefromAttack
  (params (New :type E_ActionState%20Enum :default "NewEnumerator0"))
  (return (Utilities|Array|ContainsItem (Utilities|Array|MakeArray "NewEnumerator3" "NewEnumerator4" "NewEnumerator5" "NewEnumerator6" "NewEnumerator7") New)))

(fn TransStatebyProperty
  (params (NewState :type E_ActionState%20Enum :default "NewEnumerator0"))
  (bind _controlledstateproperty (Variables|Default|GetControlledStateProperty))
  (bind _currentstate (Variables|Default|GetCurrentState))
  (bind (_value _returnvalue) (Utilities|Map|Find _controlledstateproperty _currentstate))
  (LocalVariables|SetNew NewState)
  (return (Math|Boolean|ANDBoolean _returnvalue (.ReturnValue (Utilities|Map|Find (Variables|Default|GetControlledStateProperty) (LocalVariables|GetNew))) (<= _value (.Value (Utilities|Map|Find (Variables|Default|GetControlledStateProperty) (LocalVariables|GetNew)))))))

(fn CanDodge
  (return (>= (- (Utilities|Time|GetGameTimeinSeconds) (Variables|闪避|GetLastDodgeTime)) (Variables|闪避|GetDodgeCoolDown))))

(fn CanGuard
  (return (>= (- (Utilities|Time|GetGameTimeinSeconds) (Variables|格挡|GetLastGuardEndTime)) (Variables|格挡|GetGuardCoolDown))))

(fn ForceEnterState
  (params (NewState :type E_ActionState%20Enum :default "NewEnumerator0"))
  (LocalVariables|SetNew NewState)
  (Utilities|FlowControl|Sequence
    (:then_0
      (if (not (Variables|Default|GetbCanCancel))
        (return false)))
    (:then_1
      (if (Utilities|Array|ContainsItem (Variables|Default|GetControlledState) (Variables|Default|GetCurrentState))
        (return false)))
    (:then_2
      (Variables|Default|SetCurrentState (LocalVariables|GetNew))
      (return true))))

(fn GetActionState
  (return (Variables|Default|GetCurrentState)))

(fn TryEnterState
  (params (NewState :type E_ActionState%20Enum :default "NewEnumerator0"))
  (bind _output_get (LocalVariables|SetNew NewState))
  (bind _rezult (CallFunction|CanTransitionto _output_get))
  (LocalVariables|SetCanTrans _rezult)
  (Utilities|FlowControl|Sequence
    (:then_0
      (if (LocalVariables|GetCanTrans)
        (Variables|Default|SetCurrentState (LocalVariables|GetNew))))
    (:then_1
      (return (LocalVariables|GetCanTrans)))))