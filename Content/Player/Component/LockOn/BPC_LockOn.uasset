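; Lock-on component that tracks enemies around its owner with None, Soft and Hard states.
; Each tick, a sphere overlap keeps the nearest enemy as soft target, which SimpleAimCorrect can snap yaw toward.
; Pressing hard lock pins the nearest enemy and smoothly turns owner and controller toward it.
; Hard lock drops on release, invalid target, excess distance, or when forward traces find the target behind another hit, notifying the owner except on release.
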(event Custom|UpdateSoftTarget
  (params (Actor :type Array%20of%20Actor%20Object%20References))
  ;[0.15 0.15 0.15 0.5 36] 中间事件
  (for _array_element Actor
    (if (< (Transformation|GetDistanceTo _array_element (Variables|Default|GetOwner)) (Variables|Default|GetMinMiddleVal))
      (Variables|Default|SetSoftTarget _array_element)
      (Variables|Default|SetMinMiddleVal (Transformation|GetDistanceTo _array_element (Variables|Default|GetOwner)))))
  (Variables|Default|SetMinMiddleVal 1.2e+03))

(event Custom|UpdateLockState
  (bind _owner (Variables|Default|GetOwner))
  (bind _returnvalue (Transformation|GetActorLocation _owner))
  ;[0.15 0.15 0.15 0.5 36] 中间事件
  (switch Utilities|FlowControl|Switch|SwitchonE_LockOnState (Variables|Default|GetLockState)
    (:NewEnumerator0
      (bind (_outactors _returnvalue_2) (Collision|SphereOverlapActors (Transformation|GetActorLocation (Variables|Default|GetOwner)) 1.2e+03 (Utilities|Array|MakeArray "ObjectTypeQuery8") "/Game/Enemy/BP_EnemyBase.BP_EnemyBase_C"))
      (if _returnvalue_2
        (Variables|Default|SetLockState "NewEnumerator1")
        (CallFunction|UpdateSoftTarget _outactors)
        (else
          (Variables|Default|SetSoftTarget 0))))
    (:NewEnumerator1
      (bind (_outactors_2 _returnvalue_3) (Collision|SphereOverlapActors (Transformation|GetActorLocation (Variables|Default|GetOwner)) 1.2e+03 (Utilities|Array|MakeArray "ObjectTypeQuery8") "/Game/Enemy/BP_EnemyBase.BP_EnemyBase_C"))
      (if _returnvalue_3
        (CallFunction|UpdateSoftTarget _outactors_2)
        (else
          (Variables|Default|SetLockState "NewEnumerator0")
          (Variables|Default|SetSoftTarget 0))))
    (:NewEnumerator2
      (Utilities|IsValid (Variables|Default|GetHardTarget)
        (:Is%20Valid
          (if (<= (Transformation|GetDistanceTo (Variables|Default|GetHardTarget) (Variables|Default|GetOwner)) 1.2e+03)
            (bind (_outhit _returnvalue_4) (Collision|LineTraceByChannel _returnvalue (+ _returnvalue (* (Transformation|GetActorForwardVector _owner) 3e+03)) "TraceTypeQuery1" false (Utilities|Array|MakeArray (Variables|Default|GetOwner)) "None"))
            (if _returnvalue_4
              (if (not (== (Variables|Default|GetHardTarget) (.HitActor (Collision|BreakHitResult _outhit))))
                (bind _rezult (CallFunction|IsOtherFrontOfOwner (Variables|Default|GetHardTarget)))
                (if _rezult
                  (Variables|Default|SetLockState (select (Utilities|IsValid (Variables|Default|GetSoftTarget)) "NewEnumerator1" "NewEnumerator0") :!label _label)
                  (Variables|Default|SetHardTarget 0)
                  (Class|BPIPlayer|OutHardLockState(Message) (Variables|Default|GetOwner)))))
            (else
              (goto _label))))
        (:Is%20Not%20Valid
          (goto _label))))))

(event Custom|UpdateOwnerLock
  (bind _hardtarget (Variables|Default|GetHardTarget))
  (bind _owner (Variables|Default|GetOwner))
  (bind _owner_2 (Variables|Default|GetOwner))
  (bind _delta_seconds (Variables|Default|GetDelta%20Seconds))
  (bind _owner_3 (Variables|Default|GetOwner))
  (bind _returnvalue (Transformation|GetActorRotation _owner))
  (bind _returnvalue_2 (Transformation|GetActorRotation _owner_2))
  (bind _returnvalue_3 (Transformation|GetActorLocation _owner_3))
  (bind _returnvalue_4 (Transformation|GetActorLocation _hardtarget))
  (bind _returnvalue_5 (Math|Rotator|FindLookatRotation _returnvalue_3 _returnvalue_4))
  (bind _returnvalue_6 (Math|Rotator|MakeRotator (.roll _returnvalue) (.pitch _returnvalue) (.yaw _returnvalue_5)))
  (bind _returnvalue_7 (Math|Interpolation|RInterpTo _returnvalue_2 _returnvalue_6 _delta_seconds 1e+01))
  ;[0.15 0.15 0.15 0.5 36] 中间事件
  (switch Utilities|FlowControl|Switch|SwitchonE_LockOnState (Variables|Default|GetLockState)
    (:NewEnumerator2
      (bind _as角色 (Utilities|Casting|CastToCharacter (Variables|Default|GetOwner)))
      (Pawn|SetControlRotation (Pawn|GetController _as角色) _returnvalue_7)
      (Transformation|SetActorRotation (Variables|Default|GetOwner) _returnvalue_7))))

(event EventBeginPlay
  (bind _output_get (Variables|Default|SetOwner (Components|GetOwner)))
  (bind _charactermovement (Class|BPICharacterBase|GetCharacterMovement(Message) _output_get))
  (Variables|Default|SetCharacter%20Movement _charactermovement))

(event EventTick
  (params (DeltaSeconds :type Float%20%28single-precision%29))
  (Variables|Default|SetDelta%20Seconds DeltaSeconds)
  (CallFunction|UpdateLockState)
  (CallFunction|UpdateOwnerLock))

(event EventHardLockPress
  ;[0.15 0.15 0.15 0.5 36] 接口事件
  (bind (_outactors _returnvalue) (Collision|SphereOverlapActors (Transformation|GetActorLocation (Variables|Default|GetOwner)) 1.2e+03 (Utilities|Array|MakeArray "ObjectTypeQuery8") "/Game/Enemy/BP_EnemyBase.BP_EnemyBase_C"))
  (if _returnvalue
    (CallFunction|UpdateSoftTarget _outactors)
    (Variables|Default|SetHardTarget (Variables|Default|GetSoftTarget))
    (Variables|Default|SetLockState "NewEnumerator2")))

(event EventHardLockRelease
  ;[0.15 0.15 0.15 0.5 36] 接口事件
  (Variables|Default|SetLockState (select (Utilities|IsValid (Variables|Default|GetSoftTarget)) "NewEnumerator1" "NewEnumerator0"))
  (Variables|Default|SetHardTarget 0))

(event EventSimpleAimCorrect
  ;[0.15 0.15 0.15 0.5 36] 接口事件
  (switch Utilities|FlowControl|Switch|SwitchonE_LockOnState (Variables|Default|GetLockState)
    (:NewEnumerator1
      (Utilities|IsValid (Variables|Default|GetSoftTarget)
        (:Is%20Valid
          (Transformation|SetActorRotation (Variables|Default|GetOwner) (Math|Rotator|MakeRotator 0.0 0.0 (.yaw (Math|Rotator|FindLookatRotation (Transformation|GetActorLocation (Variables|Default|GetOwner)) (Transformation|GetActorLocation (Variables|Default|GetSoftTarget)))))))
        (:Is%20Not%20Valid
          (Variables|Default|SetLockState "NewEnumerator0"))))))

(fn GetMinDistanseEnemy
  (params (Actors :type Array%20of%20Actor%20Object%20References))
  (for _array_element Actors
    (if (< (Transformation|GetDistanceTo _array_element (Variables|Default|GetOwner)) (Variables|Default|GetMinMiddleVal))
      (Variables|Default|SetSoftTarget _array_element)
      (Variables|Default|SetMinMiddleVal (Transformation|GetDistanceTo _array_element (Variables|Default|GetOwner)))))
  (Variables|Default|SetMinMiddleVal 1.2e+03))

(fn IsOtherFrontOfOwner
  (params (Actor :type Actor%20Object%20Reference))
  (bind _owner (Variables|Default|GetOwner))
  (bind _returnvalue (Transformation|GetActorLocation _owner))
  (LocalVariables|SetOwnerTarget Actor)
  (bind (_outhits _returnvalue_2) (Collision|MultiLineTraceByChannel _returnvalue (+ _returnvalue (* (Transformation|GetActorForwardVector _owner) 3e+03)) "TraceTypeQuery3" false (Utilities|Array|MakeArray (Variables|Default|GetOwner)) "Persistent"))
  (if _returnvalue_2
    (for _array_element _outhits
      (if (== (LocalVariables|GetOwnerTarget) (.HitActor (Collision|BreakHitResult _array_element)))
        (return true)))
    (return false)))

(fn GetFocusTarget
  (return (Utilities|Select :Index (Variables|Default|GetLockState) :NewEnumerator0 0 :NewEnumerator1 (Variables|Default|GetSoftTarget) :NewEnumerator2 (Variables|Default|GetHardTarget))))

(fn GetLockState
  (return (Variables|Default|GetLockState)))