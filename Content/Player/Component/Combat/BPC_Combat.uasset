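; Combat component for a character that runs data-table-driven light, heavy, dodge and jump combos, with separate ground and air moves.
; Inputs follow the current attack's Next edges, gated by the action state component, then play montages with per-move motion and gravity.
; Attack windows sweep the hitbox between frames to apply damage, knockback and feedback.
; Incoming damage plays directional light or heavy reactions; air attacks launch toward nearby lock-on targets.
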(event Custom|OnAnyMontageEnd
  (params (Montage :type Anim%20Montage%20Object%20Reference) (bInterrupted :type Boolean))
  (if (== Montage (.Montage (Utilities|Struct|BreakST_AttackData (Variables|Default|GetCuurentAttack))))
    (if (not bInterrupted)
      (CallFunction|ReliefLocomotionState))))

(event Custom|ApplyAttack
  (params (Actor :type Actor%20Object%20Reference) (HitLoc :type Vector))
  (bind _cuurentattack (Variables|Default|GetCuurentAttack))
  (bind (_id _montage _sectionstart _next _cancelstart _damagerate _poiseddamagerate _hitstop _launchenemy _canuseinair _playgravity _launchself) (Utilities|Struct|BreakST_AttackData _cuurentattack))
  ;[0.15 0.15 0.15 0.5 36] 中间事件
  (Variables|中间变量|SetMiddleActor Actor)
  (Variables|中间变量|SetMiddleVector3 HitLoc)
  (if (not (== (Variables|中间变量|GetMiddleActor) (Variables|Basic|GetOwner)))
    (Utilities|FlowControl|Sequence
      (:then_0
        (bind _attribute (Class|BPICharacterBase|GetAttributeComponent(Message) (Variables|Basic|GetOwner)))
        (bind _attack (Class|BPIAttribute|GetAttack(Message) _attribute))
        (bind _poiseattack (Class|BPIAttribute|GetPoiseAttack(Message) _attribute)))
      (:then_1
        (bind _attribute_2 (Class|BPICharacterBase|GetAttributeComponent(Message) (Variables|中间变量|GetMiddleActor)))
        (bind (_hitoutcome _bperfectblock _bisbroken _bperfectdodge) (Class|BPIAttribute|ReceiveDamage(Message) _attribute_2 (Variables|Default|GetCuurentAttack) _attack _poiseattack (Transformation|GetActorLocation (Variables|Basic|GetOwner))))
        (Variables|中间变量|SetMiddleHitOutCome _hitoutcome)
        (Variables|Default|SetPerfect%20Block _bperfectblock)
        (Variables|Default|SetbBroken _bisbroken)
        (Variables|Default|SetPerfect%20Dodge _bperfectdodge))
      (:then_3
        (bind _motor (Class|BPICharacterBase|GetMotorComponent(Message) (Variables|中间变量|GetMiddleActor)))
        (Class|BPIMotor|ApplyKnockback(Message) _motor (CallFunction|GetLaunchVector _launchenemy) false)
        (Class|BPIMotor|ApplyKnockback(Message) (Variables|Default|GetMotor) (CallFunction|GetLaunchVector _launchself) false))
      (:then_4
        (Class|BPICombatFeedBack|PlayHitFeedback(Message) (Variables|Default|GetFeedback) (Variables|中间变量|GetMiddleHitOutCome) (Variables|中间变量|GetMiddleVector3) (Variables|Default|GetPerfect%20Block) (Variables|中间变量|GetMiddleActor) (.HitStop (Utilities|Struct|BreakST_AttackData (Variables|Default|GetCuurentAttack))))))))

(event Custom|SetPropertyAfterMontage
  (bind _character_movement (Variables|Default|GetCharacter%20Movement))
  ;[0.15 0.15 0.15 0.5 36] 中间事件
  (Variables|/Script/Engine.MovementComponent|SetVelocity _character_movement (Math|Vector|MakeVector (.x (Variables|/Script/Engine.MovementComponent|GetVelocity _character_movement)) (.y (Variables|/Script/Engine.MovementComponent|GetVelocity _character_movement)) (Math|Float|Clamp(Float) (.z (Variables|/Script/Engine.MovementComponent|GetVelocity _character_movement)) -1e+04 0.0)))
  (bind _hitbox (Class|BPICharacterBase|GetHitBoxComponent(Message) (Variables|Basic|GetOwner)))
  (Utilities|IsValid _hitbox
    (:Is%20Valid
      (Variables|Default|SetPrevTraceLoc (Transformation|GetWorldLocation _hitbox)))))

(event Custom|OnDamageApplied
  (params (HitOutCome :type E_HitOutCome%20Enum :default "NewEnumerator0") (HitDirection :type E_HitDirection%20Enum :default "NewEnumerator0") (bPoiseBroken :type Boolean))
  (Variables|中间变量|SetMiddleHitOutCome HitOutCome)
  (Variables|中间变量|SetMiddleHitDirection HitDirection)
  (Variables|中间变量|SetMiddleBool bPoiseBroken)
  (if (Utilities|Enum|NotEqual(Enum) (Variables|中间变量|GetMiddleHitOutCome) "NewEnumerator0")
    (CallFunction|EnterHit (select (Variables|中间变量|GetMiddleBool) "NewEnumerator5" "NewEnumerator4") (Variables|中间变量|GetMiddleHitDirection))))

(event Custom|AirAttackAttach
  ;[0.15 0.15 0.15 0.5 36] 中间事件
  (bind _actor (Class|BPILockon|GetFocusTarget(Message) (Variables|Default|GetLock%20Component)))
  (Utilities|IsValid _actor
    (:Is%20Valid
      (Variables|Default|SetFocusTarget _actor)
      (if (Math|Float|InRange(Float) (Math|Vector|Distance(Vector) (Transformation|GetActorLocation (Variables|Default|GetFocusTarget)) (Transformation|GetActorLocation (Variables|Basic|GetOwner))) 1e+02 7e+02)
        (Character|LaunchCharacter (Variables|基本|GetOwnerCharacter) (* (Math|Vector|Normalize (Math|Vector|MakeVector (.x (- (Transformation|GetActorLocation (Variables|Default|GetFocusTarget)) (Transformation|GetActorLocation (Variables|Basic|GetOwner)))) (.y (- (Transformation|GetActorLocation (Variables|Default|GetFocusTarget)) (Transformation|GetActorLocation (Variables|Basic|GetOwner)))) (* (.z (- (Transformation|GetActorLocation (Variables|Default|GetFocusTarget)) (Transformation|GetActorLocation (Variables|Basic|GetOwner)))) 0.8))) 5e+02) false false)))))

(event Custom|PlayReactionMontage
  (params (Data :type ST%20Attack%20Data%20Structure))
  (bind (_id _montage _sectionstart _next _cancelstart _damagerate _poiseddamagerate _hitstop _launchenemy _canuseinair _playgravity _launchself _motionself _movespeed _movefriction) (Utilities|Struct|BreakST_AttackData Data))
  ;[0.15 0.15 0.15 0.5 36] 中间事件
  (Variables|中间变量|SetMiddleData Data)
  (Class|BPIMotor|SetMotionProfile(Message) (Variables|Default|GetMotor) (Utilities|Struct|MakeST_MotionProfile _movespeed _motionself _movefriction _playgravity))
  (bind _mesh (Class|BPICharacterBase|GetMeshComponent(Message) (Variables|Basic|GetOwner)))
  (Animation|Montage|PlayMontage _mesh (.Montage (Utilities|Struct|BreakST_AttackData (Variables|中间变量|GetMiddleData))) 1.0 0.0 (.SectionStart (Utilities|Struct|BreakST_AttackData (Variables|中间变量|GetMiddleData)))
    (:OnCompleted
      (CallFunction|ReliefLocomotionState))))

(event Custom|DoHitStop
  (params (D :type Float%20%28double-precision%29))
  (bind _slowtimerate (Variables|Default|GetSlowTimeRate))
  ;[0.15 0.15 0.15 0.5 36] 中间事件
  (if (not (Variables|Default|GetbInHitStop))
    (Utilities|Time|SetGlobalTimeDilation _slowtimerate)
    (Variables|Default|SetbInHitStop true)
    (Utilities|FlowControl|Delay (* D _slowtimerate))
    (Utilities|Time|SetGlobalTimeDilation 1.0)
    (Variables|Default|SetbInHitStop false)))

(event Custom|PlayMontageByID
  (params (ID :type Name))
  ;[0.15 0.15 0.15 0.5 36] 中间事件
  (bind _returnvalue (Utilities|GetDataTableRow (Variables|Basic|GetAttackDataTable) ID)
    (:then
      (Utilities|FlowControl|Sequence
        (:then_0
          (Variables|Default|SetCuurentAttack _returnvalue)
          (CallFunction|SetPropertyBeforeMontage))
        (:then_1
          (Utilities|IsValid (.Montage (Utilities|Struct|BreakST_AttackData (Variables|Default|GetCuurentAttack)))
            (:Is%20Valid
              (bind _mesh (Class|BPICharacterBase|GetMeshComponent(Message) (Variables|Basic|GetOwner)))
              (Animation|Montage|PlayMontage _mesh (.Montage (Utilities|Struct|BreakST_AttackData (Variables|Default|GetCuurentAttack))) 1.0 0.0 (.SectionStart (Utilities|Struct|BreakST_AttackData (Variables|Default|GetCuurentAttack)))))))
        (:then_2
          (CallFunction|SetPropertyAfterMontage))))))

(event Custom|OpenAttackWindow
  ;[0.15 0.15 0.15 0.5 36] 更新
  (if (Variables|Default|GetbAttackWindowOpen)
    (bind _hitbox (Class|BPICharacterBase|GetHitBoxComponent(Message) (Variables|Basic|GetOwner)))
    (bind (_outhits _returnvalue) (Class|KismetSystemLibrary|BoxTraceMulti (Variables|Default|GetPrevTraceLoc) (Transformation|GetWorldLocation _hitbox) (Components|Box|GetScaledBoxExtent _hitbox) "0, 0, 0" "TraceTypeQuery3" false (Variables|Default|GetAlreadyHit) "None" true))
    (if _returnvalue
      (for _array_element _outhits
        (if (not (or (== (Variables|Basic|GetOwner) (.HitActor (Collision|BreakHitResult _array_element))) (Utilities|Array|ContainsItem (Variables|Default|GetAlreadyHit) (.HitActor (Collision|BreakHitResult _array_element)))))
          (Utilities|Array|Add (Variables|Default|GetAlreadyHit) (.HitActor (Collision|BreakHitResult _array_element)))
          (CallFunction|ApplyAttack (.HitActor (Collision|BreakHitResult _array_element)) (.ImpactPoint (Collision|BreakHitResult _array_element))))))))

(event Custom|UpdateGravity
  ;[0.15 0.15 0.15 0.5 36] 更新
  (if (not (AI|Components|NavMovement|IsFalling (Variables|Default|GetCharacter%20Movement)))
    (if (!= (Variables|/Script/Engine.CharacterMovementComponent|GetGravityScale (Variables|Default|GetCharacter%20Movement)) 1.0)
      (Variables|/Script/Engine.CharacterMovementComponent|SetGravityScale (Variables|Default|GetCharacter%20Movement) 1.0))))

(event Custom|ReliefProperty
  ;[0.15 0.15 0.15 0.5 36] 中间事件
  (Variables|/Script/Engine.CharacterMovementComponent|SetMaxWalkSpeed (Variables|Default|GetCharacter%20Movement) (Variables|Original|GetOriginal%20Max%20Walk%20Speed))
  (Variables|/Script/Engine.CharacterMovementComponent|SetGroundFriction (Variables|Default|GetCharacter%20Movement) (Variables|Original|GetOriginal%20Ground%20Friction))
  (Variables|/Script/Engine.CharacterMovementComponent|SetMaxAcceleration (Variables|Default|GetCharacter%20Movement) (Variables|Original|GetOriginal%20Max%20Acceleration))
  (Variables|/Script/Engine.CharacterMovementComponent|SetAirControl (Variables|Default|GetCharacter%20Movement) (Variables|Original|GetOriginal%20Air%20Control))
  (Variables|/Script/Engine.CharacterMovementComponent|SetBrakingDecelerationFalling (Variables|Default|GetCharacter%20Movement) (Variables|Original|GetOriginal%20Braking%20Deceleration%20Falling)))

(event Custom|UpdateMontageMove
  (bind _cuurentattack (Variables|Default|GetCuurentAttack))
  (bind (_id _montage _sectionstart _next _cancelstart _damagerate _poiseddamagerate _hitstop _launchenemy _canuseinair _playgravity _launchself _motionself) (Utilities|Struct|BreakST_AttackData _cuurentattack))
  (bind _output (CallFunction|GetLaunchVector _motionself))
  (bind (_x _y) (Math|Vector|BreakVector _output))
  ;[0.15 0.15 0.15 0.5 36] 更新
  (Utilities|IsValid _montage
    (:Is%20Valid
      (if (Animation|Montage|MontageIsPlaying (Variables|Basic|GetAnimInst) _montage)
        (if (>= (Variables|/Script/Engine.CharacterMovementComponent|GetMaxWalkSpeed (Variables|Default|GetCharacter%20Movement)) 6.1e+02)
          (Pawn|Input|AddMovementInput (Variables|基本|GetOwnerCharacter) (Math|Vector|Normalize (Math|Vector|MakeVector _x _y 0.0)) 1.0 false))))))

(event Custom|ReliefLocomotionState
  ;[0.15 0.15 0.15 0.5 36] 中间事件
  (bind _actionstatecomponent (Class|BPIPlayer|GetActionStateComponent(Message) (Variables|Basic|GetOwner)))
  (Class|BPIActionState|SetState(Message) _actionstatecomponent "NewEnumerator0")
  (Class|BPIMotor|ResetGravity(Message) (Variables|Default|GetMotor))
  (Class|BPIPlayer|SetLockPlevisZ(Message) (Variables|Basic|GetOwner) false)
  (Variables|Default|SetCuurentAttack ""))

(event Custom|SetPropertyBeforeMontage
  (bind _cuurentattack (Variables|Default|GetCuurentAttack))
  (bind _cuurentattack_2 (Variables|Default|GetCuurentAttack))
  (bind (_id _montage _sectionstart _next _cancelstart _damagerate _poiseddamagerate _hitstop _launchenemy _canuseinair _playgravity _launchself _motionself _movespeed _movefriction _blockpelvisz) (Utilities|Struct|BreakST_AttackData _cuurentattack))
  (bind (_id_2 _montage_2 _sectionstart_2 _next_2 _cancelstart_2 _damagerate_2 _poiseddamagerate_2 _hitstop_2 _launchenemy_2 _canuseinair_2 _playgravity_2 _launchself_2 _motionself_2 _movespeed_2 _movefriction_2) (Utilities|Struct|BreakST_AttackData _cuurentattack_2))
  ;[0.15 0.15 0.15 0.5 36] 中间事件
  (Utilities|FlowControl|Sequence
    (:then_0
      (if (AI|Components|NavMovement|IsFalling (Variables|Default|GetCharacter%20Movement))
        (Variables|/Script/Engine.CharacterMovementComponent|SetAirControl (Variables|Default|GetCharacter%20Movement) 2.0)
        (Variables|/Script/Engine.CharacterMovementComponent|SetBrakingDecelerationFalling (Variables|Default|GetCharacter%20Movement) 0.0)
        (CallFunction|AirAttackAttach)))
    (:then_1
      (Variables|/Game/Player/Component/ActionState/BPC_ActionState.BPC_ActionState_C|SetbCanCancel (Variables|Default|GetAction%20State%20Component) false)
      (Variables|Default|SetbAttackWindowOpen false)
      (Utilities|Array|Clear (Variables|Default|GetAlreadyHit))
      (Class|BPIMotor|SetGravity(Message) (Variables|Default|GetMotor) _playgravity)
      (Class|BPIPlayer|SetLockPlevisZ(Message) (Variables|Basic|GetOwner) _blockpelvisz)
      (Class|BPIMotor|SetMotionProfile(Message) (Variables|Default|GetMotor) (Utilities|Struct|MakeST_MotionProfile _movespeed_2 _motionself_2 _movefriction_2 _playgravity_2)))))

(event EventBeginPlay
  (bind _mesh (Class|BPICharacterBase|GetMeshComponent(Message) (Components|GetOwner)))
  (Variables|Basic|SetAnimInst (Components|SkeletalMesh|GetAnimInstance _mesh))
  (Variables|Basic|SetOwner (Components|GetOwner))
  (EventDispatchers|BindEventtoOnMontageEnded (Variables|Basic|GetAnimInst) (delegate Custom|OnAnyMontageEnd))
  (Utilities|FlowControl|Sequence
    (:then_0
      (bind _actionstatecomponent (Class|BPIPlayer|GetActionStateComponent(Message) (Variables|Basic|GetOwner)))
      (Variables|Default|SetAction%20State%20Component _actionstatecomponent)
      (bind _charactermovement (Class|BPICharacterBase|GetCharacterMovement(Message) (Variables|Basic|GetOwner)))
      (Variables|Default|SetCharacter%20Movement _charactermovement)
      (bind _lockcomponent (Class|BPIPlayer|GetLockComponent(Message) (Variables|Basic|GetOwner)))
      (Variables|Default|SetLock%20Component _lockcomponent)
      (bind _as角色 (Utilities|Casting|CastToCharacter (Variables|Basic|GetOwner)))
      (Variables|基本|SetOwnerCharacter _as角色)
      (bind _motor (Class|BPICharacterBase|GetMotorComponent(Message) (Variables|Basic|GetOwner)))
      (Variables|Default|SetMotor _motor)
      (bind _feedback (Class|BPICharacterBase|GetCombatFeedbackComponent(Message) (Variables|Basic|GetOwner)))
      (Variables|Default|SetFeedback _feedback)
      (bind _attribute (Class|BPICharacterBase|GetAttributeComponent(Message) (Variables|Basic|GetOwner)))
      (Variables|Default|SetAttribute _attribute))
    (:then_1
      (Variables|Original|SetOriginal%20Max%20Walk%20Speed (Variables|/Script/Engine.CharacterMovementComponent|GetMaxWalkSpeed (Variables|Default|GetCharacter%20Movement)))
      (Variables|Original|SetOriginal%20Ground%20Friction (Variables|/Script/Engine.CharacterMovementComponent|GetGroundFriction (Variables|Default|GetCharacter%20Movement)))
      (Variables|Original|SetOriginal%20Max%20Acceleration (Variables|/Script/Engine.CharacterMovementComponent|GetMaxAcceleration (Variables|Default|GetCharacter%20Movement)))
      (Variables|Original|SetOriginal%20Air%20Control (Variables|/Script/Engine.CharacterMovementComponent|GetAirControl (Variables|Default|GetCharacter%20Movement)))
      (Variables|Original|SetOriginal%20Braking%20Deceleration%20Falling (Variables|/Script/Engine.CharacterMovementComponent|GetBrakingDecelerationFalling (Variables|Default|GetCharacter%20Movement))))
    (:then_2
      (EventDispatchers|BindEventtoOnDamageApplied (Variables|Default|GetAttribute) (delegate Custom|OnDamageApplied)))))

(event EventTick
  (params (DeltaSeconds :type Float%20%28single-precision%29))
  (Variables|Basic|SetDelta%20Seconds DeltaSeconds)
  (CallFunction|OpenAttackWindow)
  (CallFunction|UpdateGravity)
  (CallFunction|UpdateMontageMove))

(event EventDoLight
  ;[0.15 0.15 0.15 0.5 36] 接口事件
  (bind (_rezult _nextid) (CallFunction|HaveEdge "NewEnumerator0"))
  (if _rezult
    (bind _rezult_2 (CallFunction|IsAnimationinAir _nextid))
    (if _rezult_2
      (bind _rezult_3 (Class|BPIActionState|ForceEnterState(Message) (Variables|Default|GetAction%20State%20Component) "NewEnumerator2"))
      (if _rezult_3
        (Class|BPILockon|SimpleAimCorrect(Message) (Variables|Default|GetLock%20Component))
        (CallFunction|PlayMontagebyID _nextid)))
    (else
      (bind _rezult_4 (Class|BPIActionState|TryEnterState(Message) (Variables|Default|GetAction%20State%20Component) "NewEnumerator2"))
      (if _rezult_4
        (Class|BPILockon|SimpleAimCorrect(Message) (Variables|Default|GetLock%20Component))
        (CallFunction|PlayMontagebyID (select (AI|Components|NavMovement|IsFalling (Variables|Default|GetCharacter%20Movement)) "A_L1" "L1"))))))

(event EventOnAttackWindow
  (params (on :type Boolean))
  ;[0.15 0.15 0.15 0.5 36] 接口事件
  (bind _output_get (Variables|Default|SetbAttackWindowOpen on))
  (if _output_get
    (Utilities|Array|Clear (Variables|Default|GetAlreadyHit))
    (bind _hitbox (Class|BPICharacterBase|GetHitBoxComponent(Message) (Variables|Basic|GetOwner)))
    (Variables|Default|SetPrevTraceLoc (Transformation|GetWorldLocation _hitbox))
    (Collision|SetCollisionEnabled _hitbox "NoCollision")
    (Audio|PlaySoundatLocation "/Game/ThirdParty/Sound/SwordWhoosh.SwordWhoosh" (Variables|Default|GetPrevTraceLoc) "0, 0, 0" 0.7 1.0 0.2 0 0 0 0)))

(event EventDoDodge
  ;[0.15 0.15 0.15 0.5 36] 接口事件
  (bind (_rezult _nextid) (CallFunction|HaveEdge "NewEnumerator2"))
  (if _rezult
    (bind _rezult_2 (CallFunction|IsAnimationinAir _nextid))
    (if _rezult_2
      (if (Variables|/Game/Player/Component/ActionState/BPC_ActionState.BPC_ActionState_C|GetbCanCancel (Variables|Default|GetAction%20State%20Component))
        (bind _actionstate (Class|BPIActionState|GetActionState(Message) (Variables|Default|GetAction%20State%20Component)))
        (if (not (Utilities|Array|ContainsItem (Utilities|Array|MakeArray "NewEnumerator5" "NewEnumerator6" "NewEnumerator7") _actionstate))
          (bind _rezult_3 (Class|BPIActionState|ForceEnterState(Message) (Variables|Default|GetAction%20State%20Component) "NewEnumerator3"))
          (if _rezult_3
            (Class|BPILockon|SimpleAimCorrect(Message) (Variables|Default|GetLock%20Component))
            (CallFunction|PlayMontagebyID _nextid)))
        (else
          (bind _rezult_4 (Class|BPIActionState|CanDodge(Message) (Variables|Default|GetAction%20State%20Component) :!label _label))
          (if _rezult_4
            (bind _rezult_5 (Class|BPIActionState|TryEnterState(Message) (Variables|Default|GetAction%20State%20Component) "NewEnumerator3"))
            (if _rezult_5
              (CallFunction|PlayMontagebyID (select (AI|Components|NavMovement|IsFalling (Variables|Default|GetCharacter%20Movement)) "Dodge_F_Air" "Dodge_F"))
              (Class|BPIActionState|UpdateDodgeCD(Message) (Variables|Default|GetAction%20State%20Component) (Utilities|Time|GetGameTimeinSeconds)))))))
    (else
      (goto _label))))

(event EventDoJump
  ;[0.15 0.15 0.15 0.5 36] 接口事件
  (bind (_rezult _nextid) (CallFunction|HaveEdge "NewEnumerator3"))
  (if _rezult
    (bind _rezult_2 (CallFunction|IsAnimationinAir _nextid))
    (if _rezult_2
      (if (Variables|/Game/Player/Component/ActionState/BPC_ActionState.BPC_ActionState_C|GetbCanCancel (Variables|Default|GetAction%20State%20Component))
        (bind _actionstate (Class|BPIActionState|GetActionState(Message) (Variables|Default|GetAction%20State%20Component)))
        (if (not (Utilities|Array|ContainsItem (Utilities|Array|MakeArray "NewEnumerator5" "NewEnumerator6" "NewEnumerator7") _actionstate))
          (bind _rezult_3 (Class|BPIActionState|ForceEnterState(Message) (Variables|Default|GetAction%20State%20Component) "NewEnumerator1"))
          (if _rezult_3
            (CallFunction|PlayMontagebyID _nextid)))))
    (else
      (bind _actionstate_2 (Class|BPIActionState|GetActionState(Message) (Variables|Default|GetAction%20State%20Component)))
      (if (Utilities|Enum|Equal(Enum) _actionstate_2 "NewEnumerator0")
        (bind _rezult_4 (Class|BPIActionState|TryEnterState(Message) (Variables|Default|GetAction%20State%20Component) "NewEnumerator1"))
        (if _rezult_4
          (Class|BPIPlayer|StartJump(Message) (Variables|Basic|GetOwner)))))))

(event EventDoHeavy
  ;[0.15 0.15 0.15 0.5 36] 接口事件
  (bind (_rezult _nextid) (CallFunction|HaveEdge "NewEnumerator1"))
  (if _rezult
    (bind _rezult_2 (CallFunction|IsAnimationinAir _nextid))
    (if _rezult_2
      (bind _rezult_3 (Class|BPIActionState|ForceEnterState(Message) (Variables|Default|GetAction%20State%20Component) "NewEnumerator2"))
      (if _rezult_3
        (Class|BPILockon|SimpleAimCorrect(Message) (Variables|Default|GetLock%20Component))
        (CallFunction|PlayMontagebyID _nextid)))
    (else
      (bind _rezult_4 (Class|BPIActionState|TryEnterState(Message) (Variables|Default|GetAction%20State%20Component) "NewEnumerator2"))
      (if _rezult_4
        (Class|BPILockon|SimpleAimCorrect(Message) (Variables|Default|GetLock%20Component))
        (CallFunction|PlayMontagebyID (select (AI|Components|NavMovement|IsFalling (Variables|Default|GetCharacter%20Movement)) "AirHeavy" "H1"))))))

(event EventEnterHit
  (params (HitType :type E_ActionState%20Enum :default "NewEnumerator0") (HitLoc :type E_HitDirection%20Enum :default "NewEnumerator0"))
  ;[0.15 0.15 0.15 0.5 36] 接口事件
  (Variables|中间变量|SetMiddleActionState HitType)
  (Variables|中间变量|SetMiddleHitDirection HitLoc)
  (bind _rezult (Class|BPIActionState|TryEnterState(Message) (Variables|Default|GetAction%20State%20Component) (Variables|中间变量|GetMiddleActionState)))
  (if _rezult
    (Class|BPIActionState|SetCancelWindow(Message) (Variables|Default|GetAction%20State%20Component) false)
    (Class|BPIMotor|StopMotion(Message) (Variables|Default|GetMotor))
    (bind _returnvalue (Utilities|GetDataTableRow (Variables|Basic|GetReactionDataTable) (Select|SelectHitData (Variables|中间变量|GetMiddleActionState) (Variables|中间变量|GetMiddleHitDirection)))
      (:then
        (CallFunction|PlayReactionMontage _returnvalue)))))

(fn HaveEdge
  (params (input :type E_InputType%20Enum :default "NewEnumerator0"))
  (bind _array_element (Utilities|Array|ForEachLoopwithBreak (.Next (Utilities|Struct|BreakST_AttackData (Variables|Default|GetCuurentAttack))))
    (:LoopBody
      (if (Utilities|Enum|Equal(Enum) input (.Input (Utilities|Struct|BreakST_Edge _array_element)))
        (return true (.NextID (Utilities|Struct|BreakST_Edge _array_element)))))
    (:Completed
      (return false "None"))))

(fn GetLaunchVector
  (params (input :type Vector))
  (bind (_x _y _z) (Math|Vector|BreakVector input))
  (bind _owner (Variables|Basic|GetOwner))
  (return (+ (* (Transformation|GetActorForwardVector _owner) _x) (* (Transformation|GetActorRightVector _owner) _y) (* (Transformation|GetActorUpVector _owner) _z))))

(fn IsAnimationinAir
  (params (ID :type Name))
  (bind _returnvalue (Utilities|GetDataTableRow (Variables|Basic|GetAttackDataTable) ID)
    (:then
      (return (== (.CanUseInAir (Utilities|Struct|BreakST_AttackData _returnvalue)) (AI|Components|NavMovement|IsFalling (Variables|Default|GetCharacter%20Movement)))))))

(fn SelectHitData
  (params (ActionState :type E_ActionState%20Enum :default "NewEnumerator0") (Diection :type E_HitDirection%20Enum :default "NewEnumerator0"))
  (LocalVariables|SetState ActionState)
  (LocalVariables|SetHitDiection Diection)
  (switch Utilities|FlowControl|Switch|SwitchonE_ActionState (LocalVariables|GetState)
    (:NewEnumerator4
      (return (Utilities|Select :Index (LocalVariables|GetHitDiection) :NewEnumerator0 "HitLight_Front" :NewEnumerator1 "HitLight_Back" :NewEnumerator2 "HitLight_Left" :NewEnumerator3 "HitLight_Right")))
    (:NewEnumerator5
      (return (Utilities|Select :Index (LocalVariables|GetHitDiection) :NewEnumerator0 "HitHeavy_Front" :NewEnumerator1 "HitHeavy_Back" :NewEnumerator2 "HitHeavy_Left" :NewEnumerator3 "HitHeavy_Right")))))

(fn GetCurrentAttack
  (return (Variables|Default|GetCuurentAttack)))