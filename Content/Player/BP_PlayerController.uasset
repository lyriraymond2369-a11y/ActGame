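; Player controller that owns the player's HUD and keeps its health and posture display current.
; On possess, it fetches the pawn's attribute component through an interface message, creates the HUD widget if none exists, initializes it with that component, and adds it to the player screen.
; Tick polls the HUD to refresh every frame; a later possession does not reinitialize an existing HUD with the new attributes.
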(event EventBeginPlay)

(event EventTick
  (params (DeltaSeconds :type Float%20%28single-precision%29))
  (Class|WBPIPlayerHUD|RefreshHealthandPosture(Message) (Variables|Default|GetPlayerHUDRoot)))

(event EventPossess
  (params (PossessedPawn :type Pawn%20Object%20Reference))
  (Variables|Default|SetPossessed%20Pawn PossessedPawn)
  (Utilities|FlowControl|Sequence
    (:then_0
      (bind _attribute (Class|BPICharacterBase|GetAttributeComponent(Message) (Variables|Default|GetPossessed%20Pawn)))
      (Variables|Default|SetAttribute _attribute))
    (:then_1
      (Utilities|IsValid (Variables|Default|GetPlayerHUDRoot)
        (:Is%20Not%20Valid
          (bind _returnvalue (UserInterface|CreateWidget "/Game/Player/UI/PlayerHUD/WBP_PlayerHUD.WBP_PlayerHUD_C" self))
          (bind _output_get (Variables|Default|SetPlayerHUDRoot _returnvalue))
          (Class|WBPIPlayerHUD|InitializeHUD(Message) _output_get (Variables|Default|GetAttribute)))))
    (:then_2
      (UserInterface|Viewport|AddtoPlayerScreen (Variables|Default|GetPlayerHUDRoot)))))

(fn ConstructionScript)